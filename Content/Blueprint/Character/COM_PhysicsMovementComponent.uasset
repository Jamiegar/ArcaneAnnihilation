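; Physics-based character movement component that handles look, walk/run, jump, crouch and slide by applying forces and velocity changes to the capsule.
; It ticks during physics, running a sphere-trace ground check, extra falling gravity, drag, deceleration and sliding.
; A movement state selects drag and gates jump and slide, while slopes redirect forces along the floor plane.
; Debug prints remain, and SpeedControl is never called here.
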(event Input|EnhancedActionEvents|EnhancedInputActionIA_Look
  (params (ActionValue :type Vector%202D%20Structure) (ElapsedSeconds :type Float%20%28double-precision%29) (TriggeredSeconds :type Float%20%28double-precision%29) (InputAction :type Input%20Action%20Object%20Reference :default "/Game/Blueprint/Input/InputActions/IA_Look.IA_Look"))
  ;[0.01938 0.01938 0.01938] Mouse Camera Look
  (:Triggered
    (Pawn|Input|AddControllerYawInput (Variables|Owner|GetCharacter) (* (.x ActionValue) -1.0))
    (Pawn|Input|AddControllerPitchInput (Variables|Owner|GetCharacter) (.y ActionValue))))

(event Input|EnhancedActionEvents|EnhancedInputActionIA_Move
  (params (ActionValue :type Vector%202D%20Structure) (ElapsedSeconds :type Float%20%28double-precision%29) (TriggeredSeconds :type Float%20%28double-precision%29) (InputAction :type Input%20Action%20Object%20Reference :default "/Game/Blueprint/Input/InputActions/IA_Move.IA_Move"))
  ;[0.01938 0.01938 0.01938] Movement
  (:Triggered
    (Variables|Input|SetMovementX (.x ActionValue))
    (Variables|Input|SetMovementY (.y ActionValue))
    (Movement|Run|HandleMovement))
  (:Started
    (Variables|Input|SetMoveInput true))
  (:Completed
    (Variables|Input|SetMoveInput false)))

(event Input|EnhancedActionEvents|EnhancedInputActionIA_Jump
  (params (ActionValue :type Boolean) (ElapsedSeconds :type Float%20%28double-precision%29) (TriggeredSeconds :type Float%20%28double-precision%29) (InputAction :type Input%20Action%20Object%20Reference :default "/Game/Blueprint/Input/InputActions/IA_Jump.IA_Jump"))
  (:Triggered
    (Movement|Jump|Jump))
  (:Started
    (Variables|Movement|Jump|SetHoldingJumpInput ActionValue))
  (:Completed
    (Variables|Movement|Jump|SetHoldingJumpInput ActionValue)))

(event Input|EnhancedActionEvents|EnhancedInputActionIA_CrouchSlide
  (params (ActionValue :type Boolean) (ElapsedSeconds :type Float%20%28double-precision%29) (TriggeredSeconds :type Float%20%28double-precision%29) (InputAction :type Input%20Action%20Object%20Reference :default "/Game/Blueprint/Input/InputActions/IA_CrouchSlide.IA_CrouchSlide"))
  (:Started
    (Movement|Crouch|Crouch/Slide)))

(event EventTick
  (params (DeltaSeconds :type Float%20%28single-precision%29))
  (Movement|Jump|GroundCheck)
  (Movement|Air|ApplyFallingGravity)
  (Movement|Air|ApplyDrag)
  (CallFunction|ApplyDeaccelration)
  (Movement|Slide|SlideMovement)
  (Development|PrintString (Utilities|String|ToString(Float) (Math|Vector|VectorLength (Transformation|GetVelocity (Variables|Owner|GetCharacter)))) true true "(R=0.000000,G=0.660000,B=1.000000,A=1.000000)" 0.0))

(event EventInit
  (Components|Tick|SetTickGroup "TG_DuringPhysics")
  (bind _character (Class|BPICharacter|GetPhysicsCharacter(Message) (Components|GetOwner)))
  (bind _output_get (Variables|Owner|SetCharacter _character))
  (Class|BPIController|AddMappingContexttoPhysController(Message) (Pawn|GetController _output_get) "/Game/Blueprint/Input/IMC_Movement.IMC_Movement")
  (EventDispatchers|BindEventtoOnHitGround (EventDispatchers|CreateEvent :!event OnGrounded))
  (Variables|Movement|Crouch|SetHalfHeight (Variables|/Script/Engine.CapsuleComponent|GetCapsuleHalfHeight (Variables|/Game/Blueprint/Character/BP_PhysicsCharcter.BP_PhysicsCharcter_C|GetCapsule (Variables|Owner|GetCharacter)))))

(fn CalculateMovementDirection
  (return (+ (* (Transformation|GetActorForwardVector (Components|GetOwner)) (Variables|Input|GetMovementY)) (* (Transformation|GetActorRightVector (Components|GetOwner)) (Variables|Input|GetMovementX)))))

(fn GroundCheck
  (bind _returnvalue (Components|GetOwner))
  (bind _returnvalue_2 (Transformation|GetActorLocation _returnvalue))
  (bind (_outhit _returnvalue_3) (Collision|SphereTraceByChannel _returnvalue_2 (- (- _returnvalue_2 (Math|Vector|MakeVector 0.0 0.0 (Variables|/Script/Engine.CapsuleComponent|GetCapsuleHalfHeight (Variables|/Game/Blueprint/Character/BP_PhysicsCharcter.BP_PhysicsCharcter_C|GetCapsule (Variables|Owner|GetCharacter))))) (Math|Vector|MakeVector 0.0 0.0 (Variables|Ground|GetGround%20Check%20Distance%20Offset))) 2e+01 "TraceTypeQuery1" false 0 "None"))
  (Variables|Ground|SetFloorHit _outhit)
  (bind _output_get (Variables|Ground|SetIsGrounded _returnvalue_3))
  (if (!= _output_get (Variables|Ground|GetLastFrameGrounded))
    (if (Variables|Ground|GetIsGrounded)
      (Default|CallOnHitGround)
      (else
        (State|ChangeMovementState "NewEnumerator1"))))
  (Variables|Ground|SetLastFrameGrounded (Variables|Ground|GetIsGrounded)))

(fn Jump
  (bind _character (Variables|Owner|GetCharacter))
  (bind _returnvalue (Transformation|GetVelocity _character))
  (if (and (Variables|Movement|Jump|GetReadyToJump) (or (Utilities|Enum|Equal(Enum) (Variables|States|GetMovementState) "NewEnumerator0") (Utilities|Enum|Equal(Enum) (Variables|States|GetMovementState) "NewEnumerator3")))
    (Variables|Movement|Jump|SetReadyToJump false)
    (Variables|Movement|Run|SetExitSlope true)
    (Physics|SetPhysicsLinearVelocity (Variables|/Game/Blueprint/Character/BP_PhysicsCharcter.BP_PhysicsCharcter_C|GetCapsule _character) (Math|Vector|MakeVector (.x _returnvalue) (.y _returnvalue) 0.0) false "None")
    (Physics|AddImpulse (Variables|/Game/Blueprint/Character/BP_PhysicsCharcter.BP_PhysicsCharcter_C|GetCapsule (Variables|Owner|GetCharacter)) (* (Transformation|GetActorUpVector (Variables|Owner|GetCharacter)) (Variables|Movement|Jump|GetJumpForce)) "None" true)
    (State|ChangeMovementState "NewEnumerator1")
    (Movement|Jump|StartJumpCooldown)))

(fn ResetJump
  (Variables|Movement|Jump|SetReadyToJump true)
  (Variables|Movement|Run|SetExitSlope false))

(fn StartJumpCooldown
  (Utilities|Time|SetTimerbyEvent (EventDispatchers|CreateEvent :!event ResetJump) (Variables|Movement|Jump|GetJumpCooldown)))

(fn HandleMovement
  (bind _direction (Movement|Run|CalculateMovementDirection))
  (Physics|AddForce (Variables|/Game/Blueprint/Character/BP_PhysicsCharcter.BP_PhysicsCharcter_C|GetCapsule (Variables|Owner|GetCharacter)) (* (Math|Vector|SelectVector (Slope|GetSlopeDirection _direction) _direction (and (Slope|OnSlope) (not (Variables|Movement|Run|GetExitSlope)))) (* (Utilities|GetMovementSpeed) 1e+01)) "None" true))

(fn ApplyFallingGravity
  (if (Math|Boolean|ANDBoolean (not (Variables|Ground|GetIsGrounded)) (not (Slope|OnSlope)) (not (Variables|Movement|Jump|GetHoldingJumpInput)))
    (Physics|AddForce (Variables|/Game/Blueprint/Character/BP_PhysicsCharcter.BP_PhysicsCharcter_C|GetCapsule (Variables|Owner|GetCharacter)) (Math|Vector|MakeVector 0.0 0.0 (Variables|Movement|Air|GetFallingGravityMultiplier)) "None" true)))

(fn OnGrounded
  (State|ChangeMovementState (Variables|States|GetLastMovementState)))

(fn ApplyDrag
  (if (> (Speed|GetSpeed) 0.1)
    (Physics|AddForce (Variables|/Game/Blueprint/Character/BP_PhysicsCharcter.BP_PhysicsCharcter_C|GetCapsule (Variables|Owner|GetCharacter)) (* (* (* (Transformation|GetVelocity (Variables|Owner|GetCharacter)) (* (Utilities|Select :Index (Variables|States|GetMovementState) :NewEnumerator4 0.0 :NewEnumerator0 (Variables|Movement|Run|GetGroundDragCofficent) :NewEnumerator1 (Variables|Movement|Air|GetAirDragCofficent) :NewEnumerator2 (Variables|Movement|Crouch|GetCrouchDragCofficent) :NewEnumerator3 (Variables|Movement|Slide|GetSlideDragCofficent)) (Variables|Movement|Air|GetAirDensity))) (Variables|Movement|Air|GetReferenceArea)) -1.0) "None" true)))

(fn Crouch/Slide
  (bind _character (Variables|Owner|GetCharacter))
  (bind _character_2 (Variables|Owner|GetCharacter))
  (bind _camera (Variables|/Game/Blueprint/Character/BP_PhysicsCharcter.BP_PhysicsCharcter_C|GetCamera _character_2))
  (bind _camera_2 (Variables|/Game/Blueprint/Character/BP_PhysicsCharcter.BP_PhysicsCharcter_C|GetCamera _character))
  (if (not (Variables|Movement|Crouch|GetIsCrouched))
    (Components|Capsule|SetCapsuleHalfHeight (Variables|/Game/Blueprint/Character/BP_PhysicsCharcter.BP_PhysicsCharcter_C|GetCapsule (Variables|Owner|GetCharacter)) (Variables|Movement|Crouch|GetCrouchHalfHeight) true)
    (Transformation|SetRelativeLocation _camera (- (Variables|/Script/Engine.SceneComponent|GetRelativeLocation _camera) "0.000000,0.000000,50.000000") true false)
    (Transformation|SetActorLocation (Variables|Owner|GetCharacter) (- (Transformation|GetActorLocation (Variables|Owner|GetCharacter)) "0.000000,0.000000,50.000000") true false)
    (Variables|Movement|Crouch|SetIsCrouched true)
    (if (< (Speed|GetSpeedonXY) 2.5)
      (State|ChangeMovementState "NewEnumerator2")
      (else
        (Movement|Slide|StartSlide)))
    (elif (CallFunction|CanStand)
      (Components|Capsule|SetCapsuleHalfHeight (Variables|/Game/Blueprint/Character/BP_PhysicsCharcter.BP_PhysicsCharcter_C|GetCapsule (Variables|Owner|GetCharacter)) (Variables|Movement|Crouch|GetHalfHeight) true)
      (Transformation|SetRelativeLocation _camera_2 (+ (Variables|/Script/Engine.SceneComponent|GetRelativeLocation _camera_2) "0.000000,0.000000,50.000000") true false)
      (Transformation|SetActorLocation (Variables|Owner|GetCharacter) (+ (Transformation|GetActorLocation (Variables|Owner|GetCharacter)) "0.000000,0.000000,50.000000") true false)
      (Variables|Movement|Crouch|SetIsCrouched false)
      (State|ChangeMovementState "NewEnumerator0"))))

(fn FindGround
  (bind _returnvalue (Components|GetOwner))
  (bind _returnvalue_2 (Transformation|GetActorLocation _returnvalue))
  (bind _returnvalue_3 (Collision|SphereTraceByChannel _returnvalue_2 (+ _returnvalue_2 (* (* (Transformation|GetActorUpVector (Components|GetOwner)) -1.0) 5e+07)) 45.0 "TraceTypeQuery1" false 0 "ForOneFrame"))
  (if _returnvalue_3
    (return true (LocalVariables|GetHit))
    (else
      (return false ""))))

(fn GetSpeedonXY
  (return (Math|Vector|VectorLengthXY (Transformation|GetVelocity (Variables|Owner|GetCharacter)))))

(fn CalaculateFloorInfluence
  (params (GroundNormal :type Vector))
  (if (Utilities|Operators|EqualEqual GroundNormal (Math|Vector|VectorUp) 0.0)
    (return (Transformation|GetActorForwardVector (Variables|Owner|GetCharacter)))
    (else
      (return (Math|Vector|Normalize (Math|Vector|CrossProduct GroundNormal (Math|Vector|CrossProduct GroundNormal (Math|Vector|VectorUp))))))))

(fn ApplyDeaccelration
  (if (Math|Boolean|ANDBoolean (> (Speed|GetSpeedonXY) 0.05) (not (Variables|Input|GetMoveInput)) (Variables|Ground|GetIsGrounded) (not (Variables|Movement|Run|GetExitSlope)))
    (Utilities|MovementStateEqual "NewEnumerator3"
      (:NotEqual
        (LocalVariables|SetNewSpeed (Math|Interpolation|VInterpTo (Transformation|GetVelocity (Variables|Owner|GetCharacter)) "0, 0, 0" (Utilities|Time|GetWorldDeltaSeconds) (Variables|Movement|Run|GetDeaccelrateSpeed)))
        (Physics|SetPhysicsLinearVelocity (Variables|/Game/Blueprint/Character/BP_PhysicsCharcter.BP_PhysicsCharcter_C|GetCapsule (Variables|Owner|GetCharacter)) (* (LocalVariables|GetNewSpeed) -1.0) true "None")))))

(fn GetSpeed
  (return (Math|Vector|VectorLength (Transformation|GetVelocity (Variables|Owner|GetCharacter)))))

(fn CanStand
  (bind _character (Variables|Owner|GetCharacter))
  (bind _character_2 (Variables|Owner|GetCharacter))
  (bind _returnvalue (Transformation|GetActorLocation _character))
  (bind _capsule (Variables|/Game/Blueprint/Character/BP_PhysicsCharcter.BP_PhysicsCharcter_C|GetCapsule _character_2))
  (bind _returnvalue_2 (Components|Capsule|GetScaledCapsuleHalfHeight _capsule))
  (bind _returnvalue_3 (- _returnvalue (Math|Vector|MakeVector 0.0 0.0 _returnvalue_2)))
  (bind _returnvalue_4 (Collision|LineTraceByChannel _returnvalue_3 (+ _returnvalue_3 (Math|Vector|MakeVector 0.0 0.0 (* (Variables|Movement|Crouch|GetHalfHeight) 2.0))) "TraceTypeQuery1" false 0 "None"))
  (return (not _returnvalue_4)))

(fn OnSlope
  (bind _returnvalue (Math|Vector|VectorUp))
  (bind _floorhit (Variables|Ground|GetFloorHit))
  (bind (_bblockinghit _binitialoverlap _time _distance _location _impactpoint _normal) (Collision|BreakHitResult _floorhit))
  (bind _returnvalue_2 (Math|Vector|DotProduct _normal _returnvalue))
  (bind _returnvalue_3 (Class|KismetMathLibrary|DegAcos _returnvalue_2))
  (if _bblockinghit
    (return (and (< _returnvalue_3 (Variables|Movement|Run|GetMaxSlopeAngle)) (!= _returnvalue_3 0.0)))))

(fn GetSlopeDirection
  (params (MovementDirection :type Vector))
  (return (Math|Vector|ProjectVectorontoPlane MovementDirection (.Normal (Collision|BreakHitResult (Variables|Ground|GetFloorHit))))))

(fn StartSlide
  (State|ChangeMovementState "NewEnumerator3")
  (Variables|Movement|Slide|SetSlideTimer (Variables|Movement|Slide|GetMaxSlideTime))
  (Development|PrintString "StartSlide"))

(fn SlideMovement
  (Utilities|MovementStateEqual "NewEnumerator3"
    (:Equal
      (Development|PrintString "Slide" true true "(R=0.000000,G=0.660000,B=1.000000,A=1.000000)" 0.0)
      (if (or (not (Slope|OnSlope)) (> (.z (Transformation|GetVelocity (Variables|Owner|GetCharacter))) -0.1))
        (Physics|AddForce (Variables|/Game/Blueprint/Character/BP_PhysicsCharcter.BP_PhysicsCharcter_C|GetCapsule (Variables|Owner|GetCharacter)) (* (Movement|Run|CalculateMovementDirection) (* (Variables|Movement|Slide|GetSlideForce) 1e+01)) "None" true)
        (bind _output_get (Variables|Movement|Slide|SetSlideTimer (- (Variables|Movement|Slide|GetSlideTimer) (Utilities|Time|GetWorldDeltaSeconds))))
        (if (<= _output_get 0.0)
          (Movement|Slide|StopSliding))
        (else
          (Physics|AddForce (Variables|/Game/Blueprint/Character/BP_PhysicsCharcter.BP_PhysicsCharcter_C|GetCapsule (Variables|Owner|GetCharacter)) (* (Slope|GetSlopeDirection (Transformation|GetActorForwardVector (Variables|Owner|GetCharacter))) (* (Variables|Movement|Slide|GetSlideSlopeForce) 1e+01)) "None" true))))))

(fn StopSliding
  (State|ChangeMovementState "NewEnumerator2"))

(fn ChangeMovementState
  (params (NewState :type E_MovementState%20Enum :default "NewEnumerator0"))
  (if (Utilities|Enum|NotEqual(Enum) NewState (Variables|States|GetMovementState))
    (Variables|States|SetLastMovementState (Variables|States|GetMovementState))
    (bind _output_get (Variables|States|SetMovementState NewState))
    (Development|PrintString (Utilities|String|Append "Movement State Changed: " (Utilities|String|EnumtoString _output_get)))))

(fn SpeedControl
  (bind _character (Variables|Owner|GetCharacter))
  (bind _returnvalue (Transformation|GetVelocity _character))
  (LocalVariables|SetFlatVel (Math|Vector|MakeVector (.x _returnvalue) (.y _returnvalue) 0.0))
  (if (> (Math|Vector|VectorLength (LocalVariables|GetFlatVel)) (Utilities|GetMaxSpeedforEachState (Variables|States|GetMovementState)))
    (LocalVariables|SetLimtedVel (* (Math|Vector|Normalize (LocalVariables|GetFlatVel)) (Utilities|GetMaxSpeedforEachState (Variables|States|GetMovementState))))
    (Physics|SetPhysicsLinearVelocity (Variables|/Game/Blueprint/Character/BP_PhysicsCharcter.BP_PhysicsCharcter_C|GetCapsule (Variables|Owner|GetCharacter)) (Math|Vector|MakeVector (.x (LocalVariables|GetLimtedVel)) (.y (LocalVariables|GetLimtedVel)) (.z (Transformation|GetVelocity (Variables|Owner|GetCharacter)))) true "None")))