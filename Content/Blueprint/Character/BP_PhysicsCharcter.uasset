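; Player physics-driven character that shows the master HUD and routes shoot, interact and weapon-switch input to its components.
; On possession it initializes the physics movement state machine, adds a camera lerper component and pushes combat and additional input mapping contexts through a controller message.
; A temporary setup spawns BP_WeaponActor through a child actor with test data assets for base, barrel, stock and clip.
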(event Input|EnhancedActionEvents|EnhancedInputActionIA_Shoot
  (params (ActionValue :type Boolean) (ElapsedSeconds :type Float%20%28double-precision%29) (TriggeredSeconds :type Float%20%28double-precision%29) (InputAction :type Input%20Action%20Object%20Reference :default "/Game/Blueprint/Input/InputActions/IA_Shoot.IA_Shoot"))
  (bind _weaponactor (Variables|Default|GetWeaponActor))
  (bind _weaponcomponent (Variables|/Game/Blueprint/Weapons/BP_WeaponActor.BP_WeaponActor_C|GetWeaponComponent _weaponactor))
  (:Started
    (Default|StartAttack _weaponcomponent))
  (:Canceled
    (Default|StopAttack _weaponcomponent :!label _label))
  (:Completed
    (goto _label)))

(event Input|EnhancedActionEvents|EnhancedInputActionIA_Interact
  (params (ActionValue :type Boolean) (ElapsedSeconds :type Float%20%28double-precision%29) (TriggeredSeconds :type Float%20%28double-precision%29) (InputAction :type Input%20Action%20Object%20Reference :default "/Game/Blueprint/Input/InputActions/IA_Interact.IA_Interact"))
  (:Started
    (Default|InteractEvent (Variables|Default|GetCOM_Interact))))

(event Input|EnhancedActionEvents|EnhancedInputActionIA_SwitchWeapon
  (params (ActionValue :type Boolean) (ElapsedSeconds :type Float%20%28double-precision%29) (TriggeredSeconds :type Float%20%28double-precision%29) (InputAction :type Input%20Action%20Object%20Reference :default "/Game/Blueprint/Input/InputActions/IA_SwitchWeapon.IA_SwitchWeapon"))
  (:Started
    (Default|SwitchWeapon (Variables|Default|GetWeaponActor))))

(event EventBeginPlay
  (bind _returnvalue (UserInterface|CreateWidget "/Game/Blueprint/UI/PlayerCharacter/WBP_PlayerMaster.WBP_PlayerMaster_C"))
  (UserInterface|Viewport|AddtoViewport _returnvalue 0))

(event EventPossessed
  (params (NewController :type Controller%20Object%20Reference))
  (bind _childactor (Variables|Default|GetChildActor))
  (Class|BPIInitalizable|Init(Message) (Variables|Default|GetCOM_PhysicsMovementStateMachine))
  (bind _returnvalue (Game|AddComponentbyClass "/Game/Blueprint/Character/Camera/COM_CameraLerper.COM_CameraLerper_C" (Variables|Default|GetCamera) (Variables|Default|GetCameraContainer)))
  (Class|BPIInitalizable|Init(Message) _returnvalue)
  ;[1 1 1] WeaponSetup (temp)
  (ChildActorComponent|SetChildActorClass _childactor "/Game/Blueprint/Weapons/BP_WeaponActor.BP_WeaponActor_C")
  (bind _asbp_weapon_actor (Utilities|Casting|CastToBP_WeaponActor (Variables|/Script/Engine.ChildActorComponent|GetChildActor _childactor)))
  (Variables|/Game/Blueprint/Weapons/BP_WeaponActor.BP_WeaponActor_C|SetInitialDataAssets _asbp_weapon_actor (Utilities|Struct|MakeST_Weapon "/Game/Blueprint/Weapons/DataAssets/BaseData/DA_BaseTest1.DA_BaseTest1" "/Game/Blueprint/Weapons/DataAssets/BarrelData/DA_BarrelTest.DA_BarrelTest" "/Game/Blueprint/Weapons/DataAssets/StockData/DA_StockTest.DA_StockTest" "/Game/Blueprint/Weapons/DataAssets/ClipData/DA_ClipTest.DA_ClipTest"))
  (bind _output_get (Variables|Default|SetWeaponActor _asbp_weapon_actor))
  (Actor|SetOwner _output_get self)
  (Class|BPIInitalizable|Init(Message) _output_get)
  (Class|BPIController|AddMappingContexttoPhysController(Message) (Pawn|GetController) "/Game/Blueprint/Input/IMC_Combat.IMC_Combat" 1)
  (Class|BPIController|AddMappingContexttoPhysController(Message) (Pawn|GetController) "/Game/Blueprint/Input/IMC_AdditionalInputs.IMC_AdditionalInputs" 2))

(event Collision|EventActorBeginOverlap
  (params (OtherActor :type Actor%20Object%20Reference)))

(fn ConstructionScript)

(fn GetPhysicsCharacter
  (return self))