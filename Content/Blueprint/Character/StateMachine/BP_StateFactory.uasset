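; BP_StateFactory builds and serves the state objects for a character's movement state machine.
; On Init it constructs one object per class in InitalizableStates, passing each the state machine context and a reference to the factory.
; Each instance is cached in a map keyed by its MovementState, which GetStateOfType uses to return the existing state for a requested type.
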(event EventInit
  (CallFunction|CreateStates))

(fn CreateStates
  (for _array_element (Variables|Default|GetInitalizableStates)
    (bind _returnvalue (Game|ConstructObjectfromClass _array_element (Variables|Default|GetStateMeachineCxt) self))
    (Utilities|Map|Add (Variables|Default|GetStates) (Variables|/Game/Blueprint/Character/StateMachine/States/BP_PlayerBaseState.BP_PlayerBaseState_C|GetMovementState _returnvalue) _returnvalue)))

(fn GetStateOfType
  (params (Type :type E_PlayerMoveableStates%20Enum :default "NewEnumerator4"))
  (return (.Value (Utilities|Map|Find (Variables|Default|GetStates) Type))))