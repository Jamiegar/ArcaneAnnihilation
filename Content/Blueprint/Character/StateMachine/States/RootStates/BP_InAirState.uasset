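; Root airborne state for the character state machine, covering movement while off the ground.
; On enter it applies air drag and turns on speed-line particles, which it turns off on exit.
; Each update applies air movement and extra falling force on the capsule, and checks transitions.
; It switches state on landing, or for a wall run when a wall is hit with enough height, horizontal speed and facing alignment.
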(event EventEnterState
  (bind _statemachinecxt (Variables|Default|GetStateMachineCxt))
  (Variables|/Game/Blueprint/Character/StateMachine/COM_PhysicsMovementStateMachine.COM_PhysicsMovementStateMachine_C|SetDragCofficent _statemachinecxt (Variables|/Game/Blueprint/Character/StateMachine/COM_PhysicsMovementStateMachine.COM_PhysicsMovementStateMachine_C|GetAirDragCofficent _statemachinecxt))
  (Components|Activation|SetActive (Variables|/Game/Blueprint/Character/BP_PhysicsCharcter.BP_PhysicsCharcter_C|GetNS_SpeedLines (Default|GetPawnOwner (Variables|Default|GetStateMachineCxt))) true false))

(event EventChecktoSwitchState
  (bind _statemachinecxt (Variables|Default|GetStateMachineCxt))
  (Utilities|FlowControl|Sequence
    (:then_0
      (if (Variables|/Game/Blueprint/Character/StateMachine/COM_PhysicsMovementStateMachine.COM_PhysicsMovementStateMachine_C|GetIsGrounded (Variables|Default|GetStateMachineCxt))
        (CallFunction|SwitchState (Default|GetStateOfType (Variables|Default|GetStateFactory) "NewEnumerator2"))))
    (:then_1
      (if (Math|Boolean|ANDBoolean (or (Variables|/Game/Blueprint/Character/StateMachine/COM_PhysicsMovementStateMachine.COM_PhysicsMovementStateMachine_C|GetHitLeft _statemachinecxt) (Variables|/Game/Blueprint/Character/StateMachine/COM_PhysicsMovementStateMachine.COM_PhysicsMovementStateMachine_C|GetHitRight _statemachinecxt)) (Default|IsDistanceAboveGround (Variables|Default|GetStateMachineCxt) (Variables|/Game/Blueprint/Character/StateMachine/COM_PhysicsMovementStateMachine.COM_PhysicsMovementStateMachine_C|GetMinHeightAboveGround (Variables|Default|GetStateMachineCxt))) (>= (Math|Vector|VectorLengthXY (Transformation|GetVelocity (Default|GetPawnOwner (Variables|Default|GetStateMachineCxt)))) (Variables|/Game/Blueprint/Character/StateMachine/COM_PhysicsMovementStateMachine.COM_PhysicsMovementStateMachine_C|GetMinLinearSpeedToWallRun (Variables|Default|GetStateMachineCxt))) (CallFunction|IsCharacterFacingDirectionOfWall))
        (CallFunction|SwitchState (Default|GetStateOfType (Variables|Default|GetStateFactory) "NewEnumerator8"))))))

(event EventUpdateState
  (params (DeltaTime :type Float%20%28double-precision%29))
  (bind _statemachinecxt (Variables|Default|GetStateMachineCxt))
  (CallFunction|ChecktoSwitchState)
  (Default|ApplyMovement (Variables|Default|GetStateMachineCxt) (Variables|/Game/Blueprint/Character/StateMachine/COM_PhysicsMovementStateMachine.COM_PhysicsMovementStateMachine_C|GetMaxAirSpeed _statemachinecxt) (Variables|/Game/Blueprint/Character/StateMachine/COM_PhysicsMovementStateMachine.COM_PhysicsMovementStateMachine_C|GetMaxAirAcceleration _statemachinecxt))
  (CallFunction|ApplyFallingGravity))

(event EventExitState
  (Components|Activation|SetActive (Variables|/Game/Blueprint/Character/BP_PhysicsCharcter.BP_PhysicsCharcter_C|GetNS_SpeedLines (Default|GetPawnOwner (Variables|Default|GetStateMachineCxt))) false false))

(fn ApplyFallingGravity
  (bind _statemachinecxt (Variables|Default|GetStateMachineCxt))
  (Physics|AddForce (Variables|/Game/Blueprint/Character/BP_PhysicsCharcter.BP_PhysicsCharcter_C|GetCapsule (Default|GetPawnOwner _statemachinecxt)) (Math|Vector|MakeVector 0.0 0.0 (Variables|/Game/Blueprint/Character/StateMachine/COM_PhysicsMovementStateMachine.COM_PhysicsMovementStateMachine_C|GetFallingGravityMultiplyer _statemachinecxt)) "None" true))

(fn IsCharacterFacingDirectionOfWall
  (bind _statemachinecxt (Variables|Default|GetStateMachineCxt))
  (bind _statemachinecxt_2 (Variables|Default|GetStateMachineCxt))
  (bind _statemachinecxt_3 (Variables|Default|GetStateMachineCxt))
  (bind _return_value (Default|GetWallFoward _statemachinecxt))
  (bind _character (Default|GetPawnOwner _statemachinecxt_3))
  (bind _returnvalue (Transformation|GetActorForwardVector _character))
  (bind _returnvalue_2 (Math|Vector|DotProduct _returnvalue _return_value))
  (if (or (Variables|/Game/Blueprint/Character/StateMachine/COM_PhysicsMovementStateMachine.COM_PhysicsMovementStateMachine_C|GetHitLeft _statemachinecxt_2) (Variables|/Game/Blueprint/Character/StateMachine/COM_PhysicsMovementStateMachine.COM_PhysicsMovementStateMachine_C|GetHitRight _statemachinecxt_2))
    (Development|PrintString 0 (Utilities|String|ToString(Float) _returnvalue_2) true true "(R=0.000000,G=0.660000,B=1.000000,A=1.000000)" 0.0)
    (return (>= _returnvalue_2 0.85))))