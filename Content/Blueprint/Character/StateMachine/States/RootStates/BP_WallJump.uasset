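; Wall jump root state for a character state machine, launching the pawn up and away from a wall.
; On entry it applies a velocity-change impulse combining the pawn's up vector and the wall normal, scaled by vertical and horizontal forces from the state machine context.
; Its update checks whether the pawn is not grounded, then switches to another state obtained from the state factory.
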(event EventChecktoSwitchState
  (if (not (Variables|/Game/Blueprint/Character/StateMachine/COM_PhysicsMovementStateMachine.COM_PhysicsMovementStateMachine_C|GetIsGrounded (Variables|Default|GetStateMachineCxt)))
    (CallFunction|SwitchState (Default|GetStateOfType (Variables|Default|GetStateFactory) "NewEnumerator5"))))

(event EventUpdateState
  (params (DeltaTime :type Float%20%28double-precision%29))
  (CallFunction|ChecktoSwitchState))

(event EventEnterState
  (CallFunction|ApplyWallJump))

(fn ApplyWallJump
  (Default|AddImpulsetoPawn (Variables|Default|GetStateMachineCxt) (+ (* (Transformation|GetActorUpVector (Default|GetPawnOwner (Variables|Default|GetStateMachineCxt))) (Variables|/Game/Blueprint/Character/StateMachine/COM_PhysicsMovementStateMachine.COM_PhysicsMovementStateMachine_C|GetWallJumpVerticalForce (Variables|Default|GetStateMachineCxt))) (* (Default|GetWallNormal (Variables|Default|GetStateMachineCxt)) (Variables|/Game/Blueprint/Character/StateMachine/COM_PhysicsMovementStateMachine.COM_PhysicsMovementStateMachine_C|GetWallJumpHorzontalForce (Variables|Default|GetStateMachineCxt)))) true))