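; Grounded root state of a character's hierarchical state machine, covering movement while on the ground.
; On entry it picks a substate from movement input, applies grounded drag and plays a landing sound.
; Each update it switches states on death, lost ground or jump input, ignoring jump while moving upward on a slope.
; Crouch input is checked only during substate setup and switches states, with a further switch above a horizontal speed threshold.
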(event EventEnterState
  (params (PreviousState :type BP%20Player%20Base%20State%20Object%20Reference))
  (bind _statemachinecxt (Variables|Default|GetStateMachineCxt))
  (CallFunction|InitSubStates)
  (Variables|/Game/Blueprint/Character/StateMachine/COM_PhysicsMovementStateMachine.COM_PhysicsMovementStateMachine_C|SetDragCofficent _statemachinecxt (Variables|/Game/Blueprint/Character/StateMachine/COM_PhysicsMovementStateMachine.COM_PhysicsMovementStateMachine_C|GetGroundedDragCofficent _statemachinecxt))
  (Audio|SpawnSoundAttached "/Game/SFX/MS_Landed.MS_Landed" (Variables|/Script/Engine.Actor|GetRootComponent (Default|GetPawnOwner (Variables|Default|GetStateMachineCxt))) "None" "0, 0, 0" "0, 0, 0" "KeepRelativeOffset" false 1.0 1.0 0.0 0 0))

(event EventChecktoSwitchState
  (Utilities|FlowControl|Sequence
    (:then_0
      (if (Default|IsCharacterDead (Utilities|GetHealthComponent))
        (CallFunction|SwitchState (Default|GetStateOfType (Variables|Default|GetStateFactory) "NewEnumerator0"))))
    (:then_1
      (if (not (Variables|/Game/Blueprint/Character/StateMachine/COM_PhysicsMovementStateMachine.COM_PhysicsMovementStateMachine_C|GetIsGrounded (Variables|Default|GetStateMachineCxt)))
        (CallFunction|SwitchState (Default|GetStateOfType (Variables|Default|GetStateFactory) "NewEnumerator5"))))
    (:then_2
      (if (and (Variables|/Game/Blueprint/Character/StateMachine/COM_PhysicsMovementStateMachine.COM_PhysicsMovementStateMachine_C|GetIsJumpPressed (Variables|Default|GetStateMachineCxt)) (not (and (Default|OnSlope (Variables|Default|GetStateMachineCxt)) (> (.z (Transformation|GetVelocity (Default|GetPawnOwner (Variables|Default|GetStateMachineCxt)))) 0.1))))
        (CallFunction|SwitchState (Default|GetStateOfType (Variables|Default|GetStateFactory) "NewEnumerator3"))))))

(event EventUpdateState
  (params (DeltaTime :type Float%20%28double-precision%29))
  (CallFunction|ChecktoSwitchState))

(event EventInitSubStates
  (Utilities|FlowControl|Sequence
    (:then_0
      (if (not (Variables|/Game/Blueprint/Character/StateMachine/COM_PhysicsMovementStateMachine.COM_PhysicsMovementStateMachine_C|GetIsMovementPressed (Variables|Default|GetStateMachineCxt)))
        (CallFunction|SetSubState (Default|GetStateOfType (Variables|Default|GetStateFactory) "NewEnumerator0"))))
    (:then_1
      (if (Variables|/Game/Blueprint/Character/StateMachine/COM_PhysicsMovementStateMachine.COM_PhysicsMovementStateMachine_C|GetIsMovementPressed (Variables|Default|GetStateMachineCxt))
        (CallFunction|SetSubState (Default|GetStateOfType (Variables|Default|GetStateFactory) "NewEnumerator1"))))
    (:then_2
      (if (Variables|/Game/Blueprint/Character/StateMachine/COM_PhysicsMovementStateMachine.COM_PhysicsMovementStateMachine_C|GetCrouchPressed (Variables|Default|GetStateMachineCxt))
        (CallFunction|SwitchState (Default|GetStateOfType (Variables|Default|GetStateFactory) "NewEnumerator6"))))
    (:then_3
      (if (and (Variables|/Game/Blueprint/Character/StateMachine/COM_PhysicsMovementStateMachine.COM_PhysicsMovementStateMachine_C|GetCrouchPressed (Variables|Default|GetStateMachineCxt)) (> (Math|Vector|VectorLengthXY (Transformation|GetVelocity (Default|GetPawnOwner (Variables|Default|GetStateMachineCxt)))) 2.5))
        (CallFunction|SwitchState (Default|GetStateOfType (Variables|Default|GetStateFactory) "NewEnumerator7"))))))