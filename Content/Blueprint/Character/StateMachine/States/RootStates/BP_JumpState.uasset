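; Root jump state for the character state machine, driving a physics-simulated capsule through a jump.
; On entry it clears vertical velocity, applies an upward velocity-change impulse, flags slope exit and starts a cooldown timer for jump readiness.
; Each update applies the context's air movement and drag, and switches to another factory-provided state once the character is airborne with jump released.
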(event EventEnterState
  (CallFunction|InvokeJump))

(event EventExitState)

(event EventChecktoSwitchState
  (bind _statemachinecxt (Variables|Default|GetStateMachineCxt))
  (if (and (not (Variables|/Game/Blueprint/Character/StateMachine/COM_PhysicsMovementStateMachine.COM_PhysicsMovementStateMachine_C|GetIsGrounded _statemachinecxt)) (not (Variables|/Game/Blueprint/Character/StateMachine/COM_PhysicsMovementStateMachine.COM_PhysicsMovementStateMachine_C|GetIsJumpPressed _statemachinecxt)))
    (CallFunction|SwitchState (Default|GetStateOfType (Variables|Default|GetStateFactory) "NewEnumerator5"))))

(event EventUpdateState
  (params (DeltaTime :type Float%20%28double-precision%29))
  (bind _statemachinecxt (Variables|Default|GetStateMachineCxt))
  (bind _statemachinecxt_2 (Variables|Default|GetStateMachineCxt))
  (CallFunction|ChecktoSwitchState)
  (Default|ApplyMovement _statemachinecxt (Variables|/Game/Blueprint/Character/StateMachine/COM_PhysicsMovementStateMachine.COM_PhysicsMovementStateMachine_C|GetMaxAirSpeed _statemachinecxt) (Variables|/Game/Blueprint/Character/StateMachine/COM_PhysicsMovementStateMachine.COM_PhysicsMovementStateMachine_C|GetMaxAirAcceleration _statemachinecxt))
  (Variables|/Game/Blueprint/Character/StateMachine/COM_PhysicsMovementStateMachine.COM_PhysicsMovementStateMachine_C|SetDragCofficent _statemachinecxt_2 (Variables|/Game/Blueprint/Character/StateMachine/COM_PhysicsMovementStateMachine.COM_PhysicsMovementStateMachine_C|GetAirDragCofficent _statemachinecxt_2)))

(fn InvokeJump
  (bind _statemachinecxt (Variables|Default|GetStateMachineCxt))
  (bind _statemachinecxt_2 (Variables|Default|GetStateMachineCxt))
  (bind _statemachinecxt_3 (Variables|Default|GetStateMachineCxt))
  (bind _character (Default|GetPawnOwner _statemachinecxt_2))
  (bind _character_2 (Default|GetPawnOwner _statemachinecxt_3))
  (bind _returnvalue (Transformation|GetVelocity _character_2))
  (Variables|/Game/Blueprint/Character/StateMachine/COM_PhysicsMovementStateMachine.COM_PhysicsMovementStateMachine_C|SetReadyToJump _statemachinecxt false)
  (Variables|/Game/Blueprint/Character/StateMachine/COM_PhysicsMovementStateMachine.COM_PhysicsMovementStateMachine_C|SetExitSlope _statemachinecxt true)
  (Physics|SetPhysicsLinearVelocity (Variables|/Game/Blueprint/Character/BP_PhysicsCharcter.BP_PhysicsCharcter_C|GetCapsule _character_2) (Math|Vector|MakeVector (.x _returnvalue) (.y _returnvalue) 0.0) false "None")
  (Physics|AddImpulse (Variables|/Game/Blueprint/Character/BP_PhysicsCharcter.BP_PhysicsCharcter_C|GetCapsule _character) (* (Transformation|GetActorUpVector _character) (Variables|/Game/Blueprint/Character/StateMachine/COM_PhysicsMovementStateMachine.COM_PhysicsMovementStateMachine_C|GetJumpForce (Variables|Default|GetStateMachineCxt))) "None" true)
  (CallFunction|StartJumpCooldown))

(fn StartJumpCooldown
  (Utilities|Time|SetTimerbyEvent (EventDispatchers|CreateEvent :!event ResetJump) (Variables|/Game/Blueprint/Character/StateMachine/COM_PhysicsMovementStateMachine.COM_PhysicsMovementStateMachine_C|GetJumpCooldown (Variables|Default|GetStateMachineCxt))))

(fn ResetJump
  (bind _statemachinecxt (Variables|Default|GetStateMachineCxt))
  (Variables|/Game/Blueprint/Character/StateMachine/COM_PhysicsMovementStateMachine.COM_PhysicsMovementStateMachine_C|SetReadyToJump _statemachinecxt true)
  (Variables|/Game/Blueprint/Character/StateMachine/COM_PhysicsMovementStateMachine.COM_PhysicsMovementStateMachine_C|SetExitSlope _statemachinecxt false))