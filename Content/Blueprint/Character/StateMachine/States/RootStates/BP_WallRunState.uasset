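; Root character state machine state that drives physics-based wall running.
; On entry it keeps horizontal velocity, drops vertical speed and starts a countdown from the maximum run time.
; Each update pushes the pawn along the wall (normal cross up, flipped toward its facing) and into it, with optional wall-run gravity.
; It switches states through the factory on landing, timeout, wall loss or jump press.
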(event EventChecktoSwitchState
  (bind _statemachinecxt (Variables|Default|GetStateMachineCxt))
  (Utilities|FlowControl|Sequence
    (:then_0
      (if (Variables|/Game/Blueprint/Character/StateMachine/COM_PhysicsMovementStateMachine.COM_PhysicsMovementStateMachine_C|GetIsGrounded (Variables|Default|GetStateMachineCxt))
        (CallFunction|SwitchState (Default|GetStateOfType (Variables|Default|GetStateFactory) "NewEnumerator2"))))
    (:then_1
      (if (<= (Variables|Default|GetWallRunTimer) 0.0)
        (CallFunction|SwitchState (Default|GetStateOfType (Variables|Default|GetStateFactory) "NewEnumerator5"))))
    (:then_2
      (if (Math|Boolean|NORBoolean (Variables|/Game/Blueprint/Character/StateMachine/COM_PhysicsMovementStateMachine.COM_PhysicsMovementStateMachine_C|GetHitLeft _statemachinecxt) (Variables|/Game/Blueprint/Character/StateMachine/COM_PhysicsMovementStateMachine.COM_PhysicsMovementStateMachine_C|GetHitRight _statemachinecxt))
        (CallFunction|SwitchState (Default|GetStateOfType (Variables|Default|GetStateFactory) "NewEnumerator5"))))
    (:then_3
      (if (Variables|/Game/Blueprint/Character/StateMachine/COM_PhysicsMovementStateMachine.COM_PhysicsMovementStateMachine_C|GetIsJumpPressed (Variables|Default|GetStateMachineCxt))
        (CallFunction|SwitchState (Default|GetStateOfType (Variables|Default|GetStateFactory) "NewEnumerator9"))))))

(event EventUpdateState
  (params (DeltaTime :type Float%20%28double-precision%29))
  (CallFunction|ChecktoSwitchState)
  (CallFunction|WallRunMovement)
  (Variables|Default|SetWallRunTimer (- (Variables|Default|GetWallRunTimer) DeltaTime)))

(event EventEnterState
  (bind _statemachinecxt (Variables|Default|GetStateMachineCxt))
  (bind _character (Default|GetPawnOwner _statemachinecxt))
  (bind _returnvalue (Transformation|GetVelocity _character))
  (Physics|SetPhysicsLinearVelocity (Variables|/Game/Blueprint/Character/BP_PhysicsCharcter.BP_PhysicsCharcter_C|GetCapsule _character) (Math|Vector|MakeVector (.x _returnvalue) (.y _returnvalue) 0.0) false "None")
  (Variables|Default|SetWallRunTimer (Variables|/Game/Blueprint/Character/StateMachine/COM_PhysicsMovementStateMachine.COM_PhysicsMovementStateMachine_C|GetMaxWallRunTime (Variables|Default|GetStateMachineCxt))))

(fn WallRunMovement
  (bind _statemachinecxt (Variables|Default|GetStateMachineCxt))
  (bind _output_get (Variables|/Game/Blueprint/Character/StateMachine/COM_PhysicsMovementStateMachine.COM_PhysicsMovementStateMachine_C|SetUseGravity _statemachinecxt (Variables|/Game/Blueprint/Character/StateMachine/COM_PhysicsMovementStateMachine.COM_PhysicsMovementStateMachine_C|GetUseGravityWallRun _statemachinecxt)))
  (if _output_get
    (Default|AddForcetoOwnerPawn (Variables|Default|GetStateMachineCxt) (* (Transformation|GetActorUpVector (Default|GetPawnOwner (Variables|Default|GetStateMachineCxt))) (Variables|/Game/Blueprint/Character/StateMachine/COM_PhysicsMovementStateMachine.COM_PhysicsMovementStateMachine_C|GetWallRunGravityForce (Variables|Default|GetStateMachineCxt))) true))
  (LocalVariables|SetWallNormal (Default|GetWallNormal (Variables|Default|GetStateMachineCxt)))
  (LocalVariables|SetWallForward (Math|Vector|CrossProduct (LocalVariables|GetWallNormal) (Transformation|GetActorUpVector (Default|GetPawnOwner (Variables|Default|GetStateMachineCxt))))) ; use cross product to get the direction to travel\nalong wall
  (if (> (Math|Vector|VectorLength (- (Transformation|GetActorForwardVector (Default|GetPawnOwner (Variables|Default|GetStateMachineCxt))) (LocalVariables|GetWallForward))) (Math|Vector|VectorLength (- (Transformation|GetActorForwardVector (Default|GetPawnOwner (Variables|Default|GetStateMachineCxt))) (* (LocalVariables|GetWallForward) -1.0)))) ; True == direction of travel is closer to inverted wall forward
    (LocalVariables|SetWallForward (* (LocalVariables|GetWallForward) -1.0)))
  (Default|AddForcetoOwnerPawn (Variables|Default|GetStateMachineCxt) (* (LocalVariables|GetWallForward) (Variables|/Game/Blueprint/Character/StateMachine/COM_PhysicsMovementStateMachine.COM_PhysicsMovementStateMachine_C|GetWallRunForce (Variables|Default|GetStateMachineCxt))) true) ; Add force in direction of travel
  (Default|AddForcetoOwnerPawn (Variables|Default|GetStateMachineCxt) (* (* (LocalVariables|GetWallNormal) -1.0) 1.5e+02) true) ; Add force to stick to the wall
)