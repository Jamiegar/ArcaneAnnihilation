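; Base class for player states in a hierarchical state machine, with overridable enter, update, exit, switch-check and sub-state init hooks.
; UpdateStates updates the state and its current sub-state, while SetSubState links parent and child in both directions.
; SwitchState exits the state and its sub-state, enters the new one, then sets it on the state machine context if root, otherwise on its super state.
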(event Custom|EnterState)

(event Custom|UpdateState
  (params (DeltaTime :type Float%20%28double-precision%29)))

(event Custom|ExitState)

(event Custom|CheckToSwitchState)

(event Custom|InitSubStates)

(fn UpdateStates
  (params (DeltaTime :type Float%20%28double-precision%29))
  (CallFunction|UpdateState DeltaTime)
  (bind _currentsubstate (Variables|StateType|GetCurrentSubState)
    (:then
      (CallFunction|UpdateState _currentsubstate DeltaTime))
    (:else)))

(fn SwitchState
  (params (NewState :type BP%20Player%20Base%20State%20Object%20Reference))
  (CallFunction|ExitState) ; Exit this state
  ;[0.01938 0.01938 0.01938] Added to exit sub state
  (bind _currentsubstate (Variables|StateType|GetCurrentSubState)
    (:then
      (CallFunction|ExitState _currentsubstate) ; Exits Sub state if current state has one
    )
    (:else
      _))
  (CallFunction|EnterState NewState) ; Start the new state
  (if (Variables|StateMachine|GetIsRootState) ; Only Change StateMachine State if it is root State
    ;[0.01938 0.01938 0.01938] Switches root states
    (Default|SetCurrentState (Variables|StateMachine|GetStateMachineCxt) NewState)
    (else
      ;[0.01938 0.01938 0.01938] Switches sub states
      (bind _currentsuperstate (Variables|StateType|GetCurrentSuperState)
        (:then
          (CallFunction|SetSubState _currentsuperstate NewState))
        (:else)))))

(fn SetSuperState
  (params (NewSuperState :type BP%20Player%20Base%20State%20Object%20Reference))
  (Variables|StateType|SetCurrentSuperState NewSuperState))

(fn SetSubState
  (params (NewSubState :type BP%20Player%20Base%20State%20Object%20Reference))
  (bind _output_get (Variables|StateType|SetCurrentSubState NewSubState)) ; Set member var
  (CallFunction|SetSuperState _output_get self) ; Set the Super state to this state
)