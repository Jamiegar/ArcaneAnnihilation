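; Crouch sub-state in a character state machine, handling the pawn's lowered stance and movement.
; On enter it shrinks the capsule, lowers the camera and applies a downward force; on exit it restores capsule height and camera position.
; Each update applies crouch speed and acceleration through the state machine context, and switches state via the state factory once crouch is released and standing is possible.
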(event EventChecktoSwitchState
  (if (and (not (Variables|/Game/Blueprint/Character/StateMachine/COM_PhysicsMovementStateMachine.COM_PhysicsMovementStateMachine_C|GetCrouchPressed (Variables|Default|GetStateMachineCxt))) (Default|CanStand (Variables|Default|GetStateMachineCxt)))
    (CallFunction|SwitchState (Default|GetStateOfType (Variables|Default|GetStateFactory) "NewEnumerator0"))))

(event EventUpdateState
  (params (DeltaTime :type Float%20%28double-precision%29))
  (bind _statemachinecxt (Variables|Default|GetStateMachineCxt))
  (CallFunction|ChecktoSwitchState)
  (Default|ApplyMovement _statemachinecxt (Variables|/Game/Blueprint/Character/StateMachine/COM_PhysicsMovementStateMachine.COM_PhysicsMovementStateMachine_C|GetMaxCrouchSpeed _statemachinecxt) (Variables|/Game/Blueprint/Character/StateMachine/COM_PhysicsMovementStateMachine.COM_PhysicsMovementStateMachine_C|GetMaxCrouchAcceleration _statemachinecxt)))

(event EventEnterState
  (CallFunction|StartCrouch))

(event EventExitState
  (CallFunction|UnCrouch))

(event EventInitSubStates)

(fn StartCrouch
  (bind _statemachinecxt (Variables|Default|GetStateMachineCxt))
  (Components|Capsule|SetCapsuleHalfHeight (Variables|/Game/Blueprint/Character/BP_PhysicsCharcter.BP_PhysicsCharcter_C|GetCapsule (Default|GetPawnOwner (Variables|Default|GetStateMachineCxt))) (Variables|/Game/Blueprint/Character/StateMachine/COM_PhysicsMovementStateMachine.COM_PhysicsMovementStateMachine_C|GetCrouchHeight (Variables|Default|GetStateMachineCxt)) true)
  (Transformation|SetRelativeLocation (Variables|/Game/Blueprint/Character/BP_PhysicsCharcter.BP_PhysicsCharcter_C|GetCamera (Default|GetPawnOwner _statemachinecxt)) (- (Variables|/Game/Blueprint/Character/StateMachine/COM_PhysicsMovementStateMachine.COM_PhysicsMovementStateMachine_C|GetDefaultCameraLocation _statemachinecxt) "0.000000,0.000000,20.000000") true false)
  (Physics|AddForce (Variables|/Game/Blueprint/Character/BP_PhysicsCharcter.BP_PhysicsCharcter_C|GetCapsule (Default|GetPawnOwner (Variables|Default|GetStateMachineCxt))) "0.000000,0.000000,-2000.000000" "None" true))

(fn UnCrouch
  (Components|Capsule|SetCapsuleHalfHeight (Variables|/Game/Blueprint/Character/BP_PhysicsCharcter.BP_PhysicsCharcter_C|GetCapsule (Default|GetPawnOwner (Variables|Default|GetStateMachineCxt))) (Variables|/Game/Blueprint/Character/StateMachine/COM_PhysicsMovementStateMachine.COM_PhysicsMovementStateMachine_C|GetDefaultCapsuleHalfHeight (Variables|Default|GetStateMachineCxt)) true)
  (Transformation|SetRelativeLocation (Variables|/Game/Blueprint/Character/BP_PhysicsCharcter.BP_PhysicsCharcter_C|GetCamera (Default|GetPawnOwner (Variables|Default|GetStateMachineCxt))) (Variables|/Game/Blueprint/Character/StateMachine/COM_PhysicsMovementStateMachine.COM_PhysicsMovementStateMachine_C|GetDefaultCameraLocation (Variables|Default|GetStateMachineCxt)) true false))