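; Idle sub-state of the character state machine, active while the pawn stands still or slows to a stop.
; Each update checks for transitions, decelerates, then applies zero movement through the state machine context.
; Movement input, crouch, and crouch above a small horizontal speed each request a different state from the state factory.
; Deceleration adds a negated, interpolated velocity to the capsule's physics linear velocity.
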(event EventChecktoSwitchState
  (Utilities|FlowControl|Sequence
    (:then_0
      (if (Variables|/Game/Blueprint/Character/StateMachine/COM_PhysicsMovementStateMachine.COM_PhysicsMovementStateMachine_C|GetIsMovementPressed (Variables|Default|GetStateMachineCxt))
        (CallFunction|SwitchState (Default|GetStateOfType (Variables|Default|GetStateFactory) "NewEnumerator1"))))
    (:then_1
      (if (Variables|/Game/Blueprint/Character/StateMachine/COM_PhysicsMovementStateMachine.COM_PhysicsMovementStateMachine_C|GetCrouchPressed (Variables|Default|GetStateMachineCxt))
        (CallFunction|SwitchState (Default|GetStateOfType (Variables|Default|GetStateFactory) "NewEnumerator6"))))
    (:then_2
      (if (and (Variables|/Game/Blueprint/Character/StateMachine/COM_PhysicsMovementStateMachine.COM_PhysicsMovementStateMachine_C|GetCrouchPressed (Variables|Default|GetStateMachineCxt)) (> (Math|Vector|VectorLengthXY (Transformation|GetVelocity (Default|GetPawnOwner (Variables|Default|GetStateMachineCxt)))) 2.5))
        (CallFunction|SwitchState (Default|GetStateOfType (Variables|Default|GetStateFactory) "NewEnumerator7"))))))

(event EventUpdateState
  (params (DeltaTime :type Float%20%28double-precision%29))
  (Variables|Default|SetDelta%20Time DeltaTime)
  (CallFunction|ChecktoSwitchState)
  (CallFunction|ApplyDeaccelration)
  (Default|ApplyMovement (Variables|Default|GetStateMachineCxt) 0.0))

(fn ApplyDeaccelration
  (if (> (Default|GetSpeedXY (Variables|Default|GetStateMachineCxt)) 0.05)
    (LocalVariables|SetNewSpeed (Math|Interpolation|VInterpTo (Transformation|GetVelocity (Default|GetPawnOwner (Variables|Default|GetStateMachineCxt))) "0, 0, 0" (Variables|Default|GetDelta%20Time) (Variables|/Game/Blueprint/Character/StateMachine/COM_PhysicsMovementStateMachine.COM_PhysicsMovementStateMachine_C|GetDeaccelrationSpeed (Variables|Default|GetStateMachineCxt))))
    (Physics|SetPhysicsLinearVelocity (Variables|/Game/Blueprint/Character/BP_PhysicsCharcter.BP_PhysicsCharcter_C|GetCapsule (Default|GetPawnOwner (Variables|Default|GetStateMachineCxt))) (* (LocalVariables|GetNewSpeed) -1.0) true "None")))