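; BP_RunState is the running sub-state in a character state machine with physics-driven movement.
; Each update first switches to another factory-provided state if movement input is no longer pressed, then applies movement.
; Movement adds a mass-independent force to the pawn's capsule, scaled by run speed.
; The force follows the slope direction on slopes unless exiting one, otherwise the calculated move direction.
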(event EventUpdateState
  (params (DeltaTime :type Float%20%28double-precision%29))
  (CallFunction|ChecktoSwitchState)
  (CallFunction|ApplyMovement))

(event EventChecktoSwitchState
  (if (not (Variables|/Game/Blueprint/Character/StateMachine/COM_PhysicsMovementStateMachine.COM_PhysicsMovementStateMachine_C|GetIsMovementPressed (Variables|Default|GetStateMachineCxt)))
    (CallFunction|SwitchState (Default|GetStateOfType (Variables|Default|GetStateFactory) "NewEnumerator0"))))

(fn ApplyMovement
  (bind _statemachinecxt (Variables|Default|GetStateMachineCxt))
  (bind _statemachinecxt_2 (Variables|Default|GetStateMachineCxt))
  (bind _direction (Default|CalcMoveDirection _statemachinecxt))
  (Physics|AddForce (Variables|/Game/Blueprint/Character/BP_PhysicsCharcter.BP_PhysicsCharcter_C|GetCapsule (Default|GetPawnOwner (Variables|Default|GetStateMachineCxt))) (* (Math|Vector|SelectVector (Default|GetSlopeDirection _statemachinecxt _direction) _direction (and (Default|OnSlope _statemachinecxt_2) (not (Variables|/Game/Blueprint/Character/StateMachine/COM_PhysicsMovementStateMachine.COM_PhysicsMovementStateMachine_C|GetExitSlope _statemachinecxt_2)))) (* (Variables|/Game/Blueprint/Character/StateMachine/COM_PhysicsMovementStateMachine.COM_PhysicsMovementStateMachine_C|GetRunMovementSpeed (Variables|Default|GetStateMachineCxt)) 1e+01)) "None" true))