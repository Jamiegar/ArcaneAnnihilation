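; Slide sub-state for the character state machine, pushing the owner pawn with acceleration forces while crouch is held.
; Off slopes and not descending, it pushes along the move direction and drains a timer set from the context's max slide time.
; Otherwise it pushes along the slope direction from the actor's forward vector, without draining the timer.
; Timer expiry or crouch release requests separate follow-up states from the state factory.
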(event EventUpdateState
  (params (DeltaTime :type Float%20%28double-precision%29))
  (Variables|Default|SetDelta%20Time DeltaTime)
  (CallFunction|ChecktoSwitchState)
  (CallFunction|ApplySlideMovement))

(event EventChecktoSwitchState
  (Utilities|FlowControl|Sequence
    (:then_0
      (if (<= (Variables|Default|GetSlideTime) 0.0)
        (CallFunction|SwitchState (Default|GetStateOfType (Variables|Default|GetStateFactory) "NewEnumerator6"))))
    (:then_1
      (if (not (Variables|/Game/Blueprint/Character/StateMachine/COM_PhysicsMovementStateMachine.COM_PhysicsMovementStateMachine_C|GetCrouchPressed (Variables|Default|GetStateMachineCxt)))
        (CallFunction|SwitchState (Default|GetStateOfType (Variables|Default|GetStateFactory) "NewEnumerator0"))))))

(event EventEnterState
  (|CallParentFunction)
  (Variables|Default|SetSlideTime (Variables|/Game/Blueprint/Character/StateMachine/COM_PhysicsMovementStateMachine.COM_PhysicsMovementStateMachine_C|GetMaxSlideTime (Variables|Default|GetStateMachineCxt))))

(fn ApplySlideMovement
  (if (and (not (Default|OnSlope (Variables|Default|GetStateMachineCxt))) (> (.z (Transformation|GetVelocity (Default|GetPawnOwner (Variables|Default|GetStateMachineCxt)))) -0.1))
    (Default|AddForcetoOwnerPawn (Variables|Default|GetStateMachineCxt) (* (Default|CalcMoveDirection (Variables|Default|GetStateMachineCxt)) (* (Variables|/Game/Blueprint/Character/StateMachine/COM_PhysicsMovementStateMachine.COM_PhysicsMovementStateMachine_C|GetSlideForce (Variables|Default|GetStateMachineCxt)) 1e+01)) true)
    (CallFunction|SlideTimer)
    (else
      (Default|AddForcetoOwnerPawn (Variables|Default|GetStateMachineCxt) (* (Default|GetSlopeDirection (Variables|Default|GetStateMachineCxt) (Transformation|GetActorForwardVector (Default|GetPawnOwner (Variables|Default|GetStateMachineCxt)))) (* (Variables|/Game/Blueprint/Character/StateMachine/COM_PhysicsMovementStateMachine.COM_PhysicsMovementStateMachine_C|GetSlideSlopeForce (Variables|Default|GetStateMachineCxt)) 1e+01)) true))))

(fn SlideTimer
  (Variables|Default|SetSlideTime (- (Variables|Default|GetSlideTime) (Variables|Default|GetDelta%20Time))))