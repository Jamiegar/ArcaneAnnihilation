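; World weapon pickup that hands its weapon to the player on interact, then notifies its chest or destroys itself.
; When placed in the world without a weapon, or initialized by a chest, it builds a randomly named weapon from shuffled Asset Registry data, choosing type-compatible barrel, clip and stock.
; It previews the weapon through a child actor and stats widget.
; A detection sphere toggles the widget and the character's interact range.
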(event OnComponentBeginOverlap(DetectionSphere)
  (params (OverlappedComponent :type Primitive%20Component%20Object%20Reference) (OtherActor :type Actor%20Object%20Reference) (OtherComp :type Primitive%20Component%20Object%20Reference) (OtherBodyIndex :type Integer) (bFromSweep :type Boolean) (SweepResult :type Hit%20Result%20Structure%20%28by%20ref%29))
  (bind _character (Class|BPICharacter|GetPhysicsCharacter(Message) OtherActor))
  (Utilities|IsValid _character
    (:Is%20Valid
      (Variables|Default|SetCharacter _character)
      (Rendering|SetVisibility (Variables|Default|GetWidget) true false)
      (Default|InteractRange (Variables|/Game/Blueprint/Character/BP_PhysicsCharcter.BP_PhysicsCharcter_C|GetCOM_Interact _character)))))

(event OnComponentEndOverlap(DetectionSphere)
  (params (OverlappedComponent :type Primitive%20Component%20Object%20Reference) (OtherActor :type Actor%20Object%20Reference) (OtherComp :type Primitive%20Component%20Object%20Reference) (OtherBodyIndex :type Integer))
  (bind _character (Class|BPICharacter|GetPhysicsCharacter(Message) OtherActor))
  (Utilities|IsValid _character
    (:Is%20Valid
      (Rendering|SetVisibility (Variables|Default|GetWidget) false false)
      (Default|LeftRange (Variables|/Game/Blueprint/Character/BP_PhysicsCharcter.BP_PhysicsCharcter_C|GetCOM_Interact _character)))))

(event Custom|Init
  (params (Chest :type BP%20Chest%20Object%20Reference))
  (bind _basedata (Variables|Default|GetBaseData))
  (bind _childactor (Variables|Default|GetChildActor))
  (Variables|Default|SetChest Chest)
  (CallFunction|SelectAsset "BaseData")
  (CallFunction|SelectAsset "ClipData")
  (CallFunction|SelectAsset "BarrelData")
  (CallFunction|SelectAsset "StockData")
  (bind _output_get (Default|RandomName _basedata))
  (Variables|Default|SetWeapon (Utilities|Struct|MakeST_Weapon _basedata (Variables|Default|GetBarrelData) (Variables|Default|GetStockData) (Variables|Default|GetClipData) _output_get))
  (if (not (Variables|Default|GetActivated))
    (Variables|Default|SetActivated true)
    (ChildActorComponent|SetChildActorClass _childactor "/Game/Blueprint/Weapons/BP_WeaponActor.BP_WeaponActor_C")
    (bind _asbp_weapon_actor (Utilities|Casting|CastToBP_WeaponActor (Variables|/Script/Engine.ChildActorComponent|GetChildActor _childactor)))
    (Default|SetWeapon _asbp_weapon_actor (Variables|Default|GetWeapon))
    (bind _returnvalue (UserInterface|CreateWidget "/Game/Blueprint/Weapons/Pickup_World/W_PickupUI.W_PickupUI_C" 0 (Variables|Default|GetWeapon)))
    (UserInterface|SetWidget (Variables|Default|GetWidget) _returnvalue)
    (Default|Init _returnvalue)))

(event EventInteract
  (bind _chest (Variables|Default|GetChest))
  (bind _character (Class|BPICharacter|GetPhysicsCharacter(Message) (Pawn|GetControlledPawn (Game|GetPlayerController 0))))
  (Default|PickupWeapon (Variables|/Game/Blueprint/Character/BP_PhysicsCharcter.BP_PhysicsCharcter_C|GetWeaponActor _character) (Variables|Default|GetWeapon))
  (Utilities|IsValid _chest
    (:Is%20Valid
      (Default|Deactivate _chest self))
    (:Is%20Not%20Valid
      (Default|LeftRange (Variables|/Game/Blueprint/Character/BP_PhysicsCharcter.BP_PhysicsCharcter_C|GetCOM_Interact (Variables|Default|GetCharacter)))
      (Audio|SpawnSoundatLocation "/Game/SFX/MS_Pickup.MS_Pickup" (Transformation|GetActorLocation) "0, 0, 0" 1.0 1.0 0.0 0 0)
      (Actor|DestroyActor))))

(event EventSelected)

(event EventBeginPlay
  (bind _basedata (Variables|Default|GetBaseData))
  (bind _childactor (Variables|Default|GetChildActor))
  (if (Variables|Default|GetPlacedInWorld)
    (Utilities|FlowControl|Delay 0.5)
    (Utilities|IsValid (.BaseDataAsset (Utilities|Struct|BreakST_Weapon (Variables|Default|GetWeapon)))
      (:Is%20Valid
        _)
      (:Is%20Not%20Valid
        (CallFunction|SelectAsset "BaseData")
        (CallFunction|SelectAsset "ClipData")
        (CallFunction|SelectAsset "BarrelData")
        (CallFunction|SelectAsset "StockData")
        (bind _output_get (Default|RandomName _basedata))
        (Variables|Default|SetWeapon (Utilities|Struct|MakeST_Weapon _basedata (Variables|Default|GetBarrelData) (Variables|Default|GetStockData) (Variables|Default|GetClipData) _output_get))))
    (if (not (Variables|Default|GetActivated))
      (Variables|Default|SetActivated true)
      (ChildActorComponent|SetChildActorClass _childactor "/Game/Blueprint/Weapons/BP_WeaponActor.BP_WeaponActor_C")
      (bind _asbp_weapon_actor (Utilities|Casting|CastToBP_WeaponActor (Variables|/Script/Engine.ChildActorComponent|GetChildActor _childactor)))
      (Default|SetWeapon _asbp_weapon_actor (Variables|Default|GetWeapon))
      (bind _returnvalue (UserInterface|CreateWidget "/Game/Blueprint/Weapons/Pickup_World/W_PickupUI.W_PickupUI_C" 0 (Variables|Default|GetWeapon)))
      (UserInterface|SetWidget (Variables|Default|GetWidget) _returnvalue)
      (Default|Init _returnvalue))
    (else
      (Components|DestroyComponent (Variables|Default|GetDetectionSphere)))))

(fn ConstructionScript
  (Transformation|SetActorRotation (Math|Rotator|MakeRotator 0.0 0.0 (Math|Random|RandomFloatinRange 0.0 359.0))))

(fn SelectAsset
  (params (InputPin :type String))
  (bind _outassetdata (Class|AssetRegistry|GetAssetsbyPath (Class|AssetRegistryHelpers|GetAssetRegistry) (Utilities|String|StringToName (Utilities|String|Append "/Game/Blueprint/Weapons/DataAssets/" InputPin)) false false))
  (bind _output_get (LocalVariables|SetAssetData _outassetdata))
  (Utilities|Array|Shuffle _output_get)
  (for _array_element _output_get
    (switch string InputPin
      (:BaseData
        (bind _asda_weapon_data (Utilities|Casting|CastToDA_WeaponData (Class|AssetRegistryHelpers|GetAsset _array_element)))
        (bind _output_get_2 (Variables|Default|SetBaseData _asda_weapon_data))
        (Variables|Default|SetWeaponType (Variables|/Game/Blueprint/Weapons/DataAssets/PrimaryAssets/DA_WeaponData.DA_WeaponData_C|GetWeaponType _output_get_2)))
      (:BarrelData
        (bind _asda_barrel_attachment (Utilities|Casting|CastToDA_BarrelAttachment (Class|AssetRegistryHelpers|GetAsset _array_element)))
        (bind _success (CallFunction|TypeChecks _asda_barrel_attachment))
        (if _success
          (Utilities|IsValid (Variables|Default|GetBarrelData)
            (:Is%20Not%20Valid
              (Variables|Default|SetBarrelData _asda_barrel_attachment)))))
      (:ClipData
        (bind _asda_clip_attachment (Utilities|Casting|CastToDA_ClipAttachment (Class|AssetRegistryHelpers|GetAsset _array_element)))
        (bind _success_2 (CallFunction|TypeChecks _asda_clip_attachment))
        (if _success_2
          (Utilities|IsValid (Variables|Default|GetClipData)
            (:Is%20Not%20Valid
              (Variables|Default|SetClipData _asda_clip_attachment)))))
      (:StockData
        (bind _asda_stock_attachment (Utilities|Casting|CastToDA_StockAttachment (Class|AssetRegistryHelpers|GetAsset _array_element)))
        (bind _success_3 (CallFunction|TypeChecks _asda_stock_attachment))
        (if _success_3
          (Utilities|IsValid (Variables|Default|GetStockData)
            (:Is%20Not%20Valid
              (Variables|Default|SetStockData _asda_stock_attachment))))))))

(fn TypeChecks
  (params (Data :type DA%20Weapon%20Attachment%20Object%20Reference))
  (if (Utilities|Enum|Equal(Enum) (Variables|Default|GetWeaponType) "NewEnumerator4")
    (return true)
    (elif (or (Utilities|Enum|Equal(Enum) (Variables|/Game/Blueprint/Weapons/DataAssets/PrimaryAssets/DA_WeaponAttachment.DA_WeaponAttachment_C|GetWeaponType Data) (Variables|Default|GetWeaponType)) (Utilities|Enum|Equal(Enum) (Variables|/Game/Blueprint/Weapons/DataAssets/PrimaryAssets/DA_WeaponAttachment.DA_WeaponAttachment_C|GetWeaponType Data) "NewEnumerator4"))
      (return true)
      (else
        (return false)))))