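; Weapon reward chest that offers two pickups between waves and starts the next round once one is selected.
; Activate plays the LS_ChestOpen sequence and fades out music, then spawns two BP_BasePickup actors and enables the outline.
; Sphere overlap toggles pickup widgets and the character's interact range.
; Deactivate destroys both pickups, reverses the sequence, fades music back in and calls WaveManager.StartRound after a delay.
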(event OnComponentEndOverlap(Sphere)
  (params (OverlappedComponent :type Primitive%20Component%20Object%20Reference) (OtherActor :type Actor%20Object%20Reference) (OtherComp :type Primitive%20Component%20Object%20Reference) (OtherBodyIndex :type Integer))
  (bind _character (Class|BPICharacter|GetPhysicsCharacter(Message) OtherActor))
  (Utilities|IsValid _character
    (:Is%20Valid
      (if (Variables|Default|GetActive)
        (Rendering|SetVisibility (Variables|/Game/Blueprint/Weapons/Pickup_World/BP_BasePickup.BP_BasePickup_C|GetWidget (Variables|Default|GetPickup2)) false false)
        (Default|LeftRange (Variables|/Game/Blueprint/Character/BP_PhysicsCharcter.BP_PhysicsCharcter_C|GetCOM_Interact _character))))))

(event OnComponentBeginOverlap(Sphere)
  (params (OverlappedComponent :type Primitive%20Component%20Object%20Reference) (OtherActor :type Actor%20Object%20Reference) (OtherComp :type Primitive%20Component%20Object%20Reference) (OtherBodyIndex :type Integer) (bFromSweep :type Boolean) (SweepResult :type Hit%20Result%20Structure%20%28by%20ref%29))
  (bind _character (Class|BPICharacter|GetPhysicsCharacter(Message) OtherActor))
  (Utilities|IsValid _character
    (:Is%20Valid
      (Variables|Default|SetCharacter _character)
      (if (Variables|Default|GetActive)
        (Rendering|SetVisibility (Variables|/Game/Blueprint/Weapons/Pickup_World/BP_BasePickup.BP_BasePickup_C|GetWidget (Variables|Default|GetPickup1)) true false)
        (Default|InteractRange (Variables|/Game/Blueprint/Character/BP_PhysicsCharcter.BP_PhysicsCharcter_C|GetCOM_Interact _character) self)))))

(event Custom|Activate
  (params (WaveManager :type BP%20Wave%20Manager%20Object%20Reference))
  (bind _returnvalue (Sequencer|Player|CreateLevelSequencePlayer "/Game/Blueprint/LevelElements/Sequence/LS_ChestOpen.LS_ChestOpen"))
  (Sequencer|Player|Play _returnvalue :!class /Script/MovieScene.MovieSceneSequencePlayer)
  (EventDispatchers|AssignOnFinished _returnvalue (delegate Custom|OnFinished_Event))
  (bind _gamemode (Class|BPIArcaneGM|GetArcaneGameMode(Message) (Game|GetGameMode)))
  (Default|FadeOutTitleMusic _gamemode)
  (if (not (== (Utilities|GetClass self) "/Game/Blueprint/Weapons/Pickup_World/BP_MenuChest.BP_MenuChest_C"))
    (Audio|PlaySound2D "/Game/ExternalAssets_Ungraded/FreeSound/Chest_SC.Chest_SC" 1.0 1.0 0.0 0 0)))

(event Custom|Deactivate
  (params (SelectedWeapon :type BP%20Base%20Pickup%20Object%20Reference))
  (Variables|Default|SetActive false)
  (Actor|DestroyActor (Variables|Default|GetPickup1)) ; temp
  (Rendering|SetRenderCustomDepth (Variables|Default|GetChest_Base_0) false)
  (Default|LeftRange (Variables|/Game/Blueprint/Character/BP_PhysicsCharcter.BP_PhysicsCharcter_C|GetCOM_Interact (Variables|Default|GetCharacter)))
  (Utilities|FlowControl|Sequence
    (:then_0
      (Utilities|FlowControl|Delay 2.0)
      (Default|StartRound (Variables|Default|GetWaveManager)))
    (:then_1
      (bind _returnvalue (Sequencer|Player|CreateLevelSequencePlayer "/Game/Blueprint/LevelElements/Sequence/LS_ChestOpen.LS_ChestOpen"))
      (Class|MovieSceneSequencePlayer|PlayReverse _returnvalue)
      (EventDispatchers|AssignOnFinished _returnvalue (delegate Custom|OnFinished_Event_0)))))

(event Custom|OnFinished_Event
  (Transformation|SetRelativeLocation (Variables|Default|GetChest_Lid) "-50.000000,0.000000,17.536713" false false)
  (Variables|Default|SetWaveManager (stale Custom|Activate WaveManager))
  (if (not (Variables|Default|GetActive))
    (Variables|Default|SetActive true)
    (Rendering|SetRenderCustomDepth (Variables|Default|GetChest_Base_0) true)
    (Utilities|IsValid (Variables|Default|GetPickup1)
      (:Is%20Valid
        _)
      (:Is%20Not%20Valid
        (bind _returnvalue (Game|SpawnActorfromClass "/Game/Blueprint/Weapons/Pickup_World/BP_BasePickup.BP_BasePickup_C" (Math|Transform|MakeTransform (Transformation|GetWorldLocation (Variables|Default|GetWeapon1)) "0, 0, 0" "1.000000,1.000000,1.000000") "Undefined" 0 0))
        (bind _output_get (Variables|Default|SetPickup1 _returnvalue))
        (Default|Init _output_get self)))
    (Utilities|IsValid (Variables|Default|GetPickup2)
      (:Is%20Not%20Valid
        (bind _returnvalue_2 (Game|SpawnActorfromClass "/Game/Blueprint/Weapons/Pickup_World/BP_BasePickup.BP_BasePickup_C" (Math|Transform|MakeTransform (Transformation|GetWorldLocation (Variables|Default|GetWeapon2)) "0, 0, 0" "1.000000,1.000000,1.000000") "Undefined" 0 0))
        (bind _output_get_2 (Variables|Default|SetPickup2 _returnvalue_2))
        (Default|Init _output_get_2 self)))))

(event Custom|OnFinished_Event_0
  (Transformation|SetRelativeLocation (Variables|Default|GetChest_Lid) "-50.000000,0.000000,-90.000000" false false)
  (bind _gamemode (Class|BPIArcaneGM|GetArcaneGameMode(Message) (Game|GetGameMode)))
  (Default|FadeinTileMusic _gamemode))

(fn ConstructionScript)