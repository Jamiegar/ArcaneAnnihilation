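; Menu variant of a weapon chest that re-arms itself after each selection.
; BeginPlay is overridden empty, so the chest does not call Activate on start.
; Deactivate hides both pickup widgets, destroys the selected weapon actor, clears Active and tells the character's interact component it left range.
; After a short delay it calls Activate again, making the chest reusable.
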(event EventBeginPlay
  ;[1 1 1] stop that
)

(event EventDeactivate
  (params (SelectedWeapon :type BP%20Base%20Pickup%20Object%20Reference))
  (Rendering|SetVisibility (Variables|/Game/Blueprint/Weapons/Pickup_World/BP_BasePickup.BP_BasePickup_C|GetWidget (Variables|Default|GetPickup2)) false false)
  (Actor|DestroyActor SelectedWeapon)
  (Variables|Default|SetActive false)
  (Default|LeftRange (Variables|/Game/Blueprint/Character/BP_PhysicsCharcter.BP_PhysicsCharcter_C|GetCOM_Interact (Variables|Default|GetCharacter)))
  (Utilities|FlowControl|Delay 2.0)
  (CallFunction|Activate))

(fn ConstructionScript
  (|CallParentFunction))