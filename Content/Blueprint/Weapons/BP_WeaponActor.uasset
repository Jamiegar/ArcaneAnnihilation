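; Modular weapon actor that builds its owning character's gun from base, barrel, clip and stock data assets.
; SetWeapon checks that part types match, with one enum value as wildcard, then spawns the base's weapon component, copies stats onto it and snaps part meshes to base sockets.
; It keeps current and stored weapons with separate ammo counts, swapping them on switch.
; Pickups overwrite the stored slot and trigger the character's swap; switching and reloading update the ammo UI.
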(event Custom|SwitchWeapon
  (Variables|/Game/Blueprint/Character/BP_PhysicsCharcter.BP_PhysicsCharcter_C|SetSwapping (Variables|Default|GetCharacter) false)
  (CallFunction|SwitchVariables0)
  (CallFunction|SetWeapon (Variables|Default|GetStoredWeapon))
  (CallFunction|SwitchVariables)
  (CallFunction|UpdateAmmoUI))

(event Custom|SetWeapon
  (params (ST_ChosenDataAssets :type ST%20Weapon%20Structure%20%28by%20ref%29))
  (bind (_basedataasset _barreldataasset _stockdataasset _clipdataasset) (Utilities|Struct|BreakST_Weapon ST_ChosenDataAssets))
  (Variables|Default|SetWeaponBase _basedataasset)
  (Variables|Default|SetBarrel _barreldataasset)
  (Variables|Default|SetStock _stockdataasset)
  (Variables|Default|SetClip _clipdataasset)
  (bind _fuckingworked (CallFunction|TypeChecks))
  (if _fuckingworked
    (CallFunction|SetBase)
    (CallFunction|SetBarrel)
    (CallFunction|SetClip)
    (CallFunction|SetStock)
    (Default|Init (Variables|Default|GetWeaponComponent))
    (else
      (Development|PrintString "U fucked it mororn"))))

(event Custom|PickupWeapon
  (params (Weapon :type ST%20Weapon%20Structure))
  (bind _output_get (Variables|Default|SetStoredWeapon Weapon))
  (Variables|Default|SetStoredAmmo (Variables|/Game/Blueprint/Weapons/DataAssets/PrimaryAssets/DA_ClipAttachment.DA_ClipAttachment_C|GetMagazineSize (.ClipDataAsset (Utilities|Struct|BreakST_Weapon _output_get))))
  (Default|StopAttack (Variables|Default|GetWeaponComponent))
  (Default|CallOnSwapWeapon (Variables|Default|GetCharacter)))

(event Custom|Reload
  (bind _weaponcomponent (Variables|Default|GetWeaponComponent))
  (Variables|/Game/Blueprint/Weapons/Components/COM_BaseWeaponLogic.COM_BaseWeaponLogic_C|SetCurrentAmmo _weaponcomponent (Variables|/Game/Blueprint/Weapons/Components/COM_BaseWeaponLogic.COM_BaseWeaponLogic_C|GetMagazineSize _weaponcomponent))
  (CallFunction|UpdateAmmoUI))

(event EventInit
  (bind _initialdataassets (Variables|Default|GetInitialDataAssets))
  (bind _output_get (Variables|Default|SetCurrentWeapon _initialdataassets))
  (Variables|Default|SetCurentAmmo (Variables|/Game/Blueprint/Weapons/DataAssets/PrimaryAssets/DA_ClipAttachment.DA_ClipAttachment_C|GetMagazineSize (.ClipDataAsset (Utilities|Struct|BreakST_Weapon _initialdataassets))))
  (CallFunction|SetWeapon _output_get)
  (bind _character (Class|BPICharacter|GetPhysicsCharacter(Message) (Components|GetOwner)))
  (bind _output_get_2 (Variables|Default|SetCharacter _character))
  (EventDispatchers|BindEventtoOnWeaponSwapped _output_get_2 (EventDispatchers|CreateEvent :!event Custom|SwitchWeapon)))

(fn ConstructionScript)

(fn SetBase
  (bind _weaponbase (Variables|Default|GetWeaponBase))
  (bind _weaponbase_2 (Variables|Default|GetWeaponBase))
  (bind _basemesh (Variables|Default|GetBaseMesh))
  (Utilities|IsValid (Variables|Default|GetWeaponComponent)
    (:Is%20Valid
      (Components|DestroyComponent (Variables|Default|GetWeaponComponent)))
    (:Is%20Not%20Valid
      _))
  (bind _returnvalue (Game|AddComponentbyClass (Variables|/Game/Blueprint/Weapons/DataAssets/PrimaryAssets/DA_WeaponData.DA_WeaponData_C|GetWeaponComponent (Variables|Default|GetWeaponBase)) self))
  (Variables|Default|SetWeaponComponent _returnvalue)
  (Components|StaticMesh|SetStaticMesh _basemesh (Variables|/Game/Blueprint/Weapons/DataAssets/PrimaryAssets/DA_WeaponData.DA_WeaponData_C|GetBaseWeapon _weaponbase_2))
  (Rendering|Material|SetMaterial _basemesh 0 (Variables|/Game/Blueprint/Weapons/DataAssets/PrimaryAssets/DA_WeaponData.DA_WeaponData_C|GetMaterial _weaponbase_2))
  (Variables|/Game/Blueprint/Weapons/Components/COM_BaseWeaponLogic.COM_BaseWeaponLogic_C|SetDamage (Variables|Default|GetWeaponComponent) (Variables|/Game/Blueprint/Weapons/DataAssets/PrimaryAssets/DA_WeaponData.DA_WeaponData_C|GetDamage _weaponbase))
  (Variables|/Game/Blueprint/Weapons/Components/COM_BaseWeaponLogic.COM_BaseWeaponLogic_C|SetFireRate (Variables|Default|GetWeaponComponent) (Variables|/Game/Blueprint/Weapons/DataAssets/PrimaryAssets/DA_WeaponData.DA_WeaponData_C|GetFireRate _weaponbase))
  (Variables|/Game/Blueprint/Weapons/Components/COM_BaseWeaponLogic.COM_BaseWeaponLogic_C|SetAutomatic (Variables|Default|GetWeaponComponent) (Variables|/Game/Blueprint/Weapons/DataAssets/PrimaryAssets/DA_WeaponData.DA_WeaponData_C|GetAutomatic _weaponbase))
  (Variables|/Game/Blueprint/Weapons/Components/COM_BaseWeaponLogic.COM_BaseWeaponLogic_C|SetProjectile (Variables|Default|GetWeaponComponent) (Variables|/Game/Blueprint/Weapons/DataAssets/PrimaryAssets/DA_WeaponData.DA_WeaponData_C|GetProjectiletoSpawn _weaponbase))
  (Variables|/Game/Blueprint/Weapons/Components/COM_BaseWeaponLogic.COM_BaseWeaponLogic_C|SetFireSound (Variables|Default|GetWeaponComponent) (Variables|/Game/Blueprint/Weapons/DataAssets/PrimaryAssets/DA_WeaponData.DA_WeaponData_C|GetFireSound _weaponbase)))

(fn SetBarrel
  (bind _barrel (Variables|Default|GetBarrel))
  (bind _barrel_2 (Variables|Default|GetBarrel))
  (bind _weaponcomponent (Variables|Default|GetWeaponComponent))
  (CallFunction|SetMesh (Variables|Default|GetBarrel) (Variables|Default|GetBarrelMesh))
  (Transformation|SetRelativeLocation (Variables|Default|GetFirePoint) (Variables|/Game/Blueprint/Weapons/DataAssets/PrimaryAssets/DA_BarrelAttachment.DA_BarrelAttachment_C|GetFirePointLocation _barrel_2) false false)
  (Variables|/Game/Blueprint/Weapons/Components/COM_BaseWeaponLogic.COM_BaseWeaponLogic_C|SetRange _weaponcomponent (Variables|/Game/Blueprint/Weapons/DataAssets/PrimaryAssets/DA_BarrelAttachment.DA_BarrelAttachment_C|GetRange _barrel))
  (Variables|/Game/Blueprint/Weapons/Components/COM_BaseWeaponLogic.COM_BaseWeaponLogic_C|SetProjectileColour _weaponcomponent (Variables|/Game/Blueprint/Weapons/DataAssets/PrimaryAssets/DA_BarrelAttachment.DA_BarrelAttachment_C|GetProjectileColour _barrel))
  (Variables|/Game/Blueprint/Weapons/Components/COM_BaseWeaponLogic.COM_BaseWeaponLogic_C|SetProjectileSize _weaponcomponent (Variables|/Game/Blueprint/Weapons/DataAssets/PrimaryAssets/DA_BarrelAttachment.DA_BarrelAttachment_C|GetProjectileSize _barrel_2)))

(fn SetClip
  (bind _clip (Variables|Default|GetClip))
  (bind _weaponcomponent (Variables|Default|GetWeaponComponent))
  (CallFunction|SetMesh (Variables|Default|GetClip) (Variables|Default|GetClipMesh))
  (Variables|/Game/Blueprint/Weapons/Components/COM_BaseWeaponLogic.COM_BaseWeaponLogic_C|SetDamageMultiplier _weaponcomponent (Variables|/Game/Blueprint/Weapons/DataAssets/PrimaryAssets/DA_ClipAttachment.DA_ClipAttachment_C|GetDamageMultiplier _clip))
  (Variables|/Game/Blueprint/Weapons/Components/COM_BaseWeaponLogic.COM_BaseWeaponLogic_C|SetMagazineSize _weaponcomponent (Variables|/Game/Blueprint/Weapons/DataAssets/PrimaryAssets/DA_ClipAttachment.DA_ClipAttachment_C|GetMagazineSize _clip))
  (Variables|/Game/Blueprint/Weapons/Components/COM_BaseWeaponLogic.COM_BaseWeaponLogic_C|SetCurrentAmmo _weaponcomponent (Variables|Default|GetCurentAmmo))
  (Variables|/Game/Blueprint/Weapons/Components/COM_BaseWeaponLogic.COM_BaseWeaponLogic_C|SetReloadTime _weaponcomponent (Variables|/Game/Blueprint/Weapons/DataAssets/PrimaryAssets/DA_ClipAttachment.DA_ClipAttachment_C|GetReloadTime _clip))
  (Variables|/Game/Blueprint/Weapons/Components/COM_BaseWeaponLogic.COM_BaseWeaponLogic_C|SetProjectileSpeed _weaponcomponent (Variables|/Game/Blueprint/Weapons/DataAssets/PrimaryAssets/DA_ClipAttachment.DA_ClipAttachment_C|GetProjectileSpeed _clip))
  (Variables|/Game/Blueprint/Weapons/Components/COM_BaseWeaponLogic.COM_BaseWeaponLogic_C|SetBounceAmount _weaponcomponent (Variables|/Game/Blueprint/Weapons/DataAssets/PrimaryAssets/DA_ClipAttachment.DA_ClipAttachment_C|GetBounceAmount _clip)))

(fn SetStock
  (bind _weaponcomponent (Variables|Default|GetWeaponComponent))
  (CallFunction|SetMesh (Variables|Default|GetStock) (Variables|Default|GetStockMesh))
  (Variables|/Game/Blueprint/Weapons/Components/COM_BaseWeaponLogic.COM_BaseWeaponLogic_C|SetAccuracy _weaponcomponent (Variables|/Game/Blueprint/Weapons/DataAssets/PrimaryAssets/DA_StockAttachment.DA_StockAttachment_C|GetAccuracyModifier (Variables|Default|GetStock)))
  ;[1 1 1] player shit
  (Variables|/Game/Blueprint/Weapons/Components/COM_BaseWeaponLogic.COM_BaseWeaponLogic_C|SetRecoilAmount _weaponcomponent (Variables|/Game/Blueprint/Weapons/DataAssets/PrimaryAssets/DA_StockAttachment.DA_StockAttachment_C|GetRecoilAmount (Variables|Default|GetStock))))

(fn SetMesh
  (params (Data :type DA%20Weapon%20Attachment%20Object%20Reference) (Mesh :type Static%20Mesh%20Component%20Object%20Reference))
  (Components|StaticMesh|SetStaticMesh Mesh (Variables|/Game/Blueprint/Weapons/DataAssets/PrimaryAssets/DA_WeaponAttachment.DA_WeaponAttachment_C|GetAttachmentMesh Data))
  (Rendering|Material|SetMaterial Mesh 0 (Variables|/Game/Blueprint/Weapons/DataAssets/PrimaryAssets/DA_WeaponAttachment.DA_WeaponAttachment_C|GetMaterial Data))
  (Transformation|AttachComponentToComponent Mesh (Variables|Default|GetBaseMesh) (Variables|/Game/Blueprint/Weapons/DataAssets/PrimaryAssets/DA_WeaponAttachment.DA_WeaponAttachment_C|GetSocketName Data) "SnapToTarget" "SnapToTarget" "SnapToTarget" true))

(fn TypeChecks
  (bind _barrel (Variables|Default|GetBarrel))
  (bind _stock (Variables|Default|GetStock))
  (bind _clip (Variables|Default|GetClip))
  (bind _weaponbase (Variables|Default|GetWeaponBase))
  (bind _weapontype (Variables|/Game/Blueprint/Weapons/DataAssets/PrimaryAssets/DA_WeaponAttachment.DA_WeaponAttachment_C|GetWeaponType _barrel))
  (bind _weapontype_2 (Variables|/Game/Blueprint/Weapons/DataAssets/PrimaryAssets/DA_WeaponAttachment.DA_WeaponAttachment_C|GetWeaponType _stock))
  (bind _weapontype_3 (Variables|/Game/Blueprint/Weapons/DataAssets/PrimaryAssets/DA_WeaponAttachment.DA_WeaponAttachment_C|GetWeaponType _clip))
  (bind _weapontype_4 (Variables|/Game/Blueprint/Weapons/DataAssets/PrimaryAssets/DA_WeaponData.DA_WeaponData_C|GetWeaponType _weaponbase))
  (if (Utilities|Enum|Equal(Enum) _weapontype_4 "NewEnumerator4")
    (return true)
    (else
      (if (Utilities|Enum|Equal(Enum) _weapontype_4 _weapontype)
        _
        (elif (Utilities|Enum|Equal(Enum) _weapontype "NewEnumerator4")
          _
          (else
            (return false))))
      (if (Utilities|Enum|Equal(Enum) (Variables|/Game/Blueprint/Weapons/DataAssets/PrimaryAssets/DA_WeaponData.DA_WeaponData_C|GetWeaponType (Variables|Default|GetWeaponBase)) _weapontype_2)
        _
        (elif (Utilities|Enum|Equal(Enum) _weapontype_2 "NewEnumerator4")
          _
          (else
            (return false))))
      (if (Utilities|Enum|Equal(Enum) (Variables|/Game/Blueprint/Weapons/DataAssets/PrimaryAssets/DA_WeaponData.DA_WeaponData_C|GetWeaponType (Variables|Default|GetWeaponBase)) _weapontype_3)
        _
        (elif (Utilities|Enum|Equal(Enum) _weapontype_3 "NewEnumerator4")
          _
          (else
            (return false))))
      (return true))))

(fn SwitchVariables
  (LocalVariables|SetTempVairable (Variables|Default|GetStoredWeapon))
  (Variables|Default|SetStoredWeapon (Variables|Default|GetCurrentWeapon))
  (Variables|Default|SetCurrentWeapon (LocalVariables|GetTempVairable)))

(fn SwitchVariables0
  (LocalVariables|SetTemp (Variables|/Game/Blueprint/Weapons/Components/COM_BaseWeaponLogic.COM_BaseWeaponLogic_C|GetCurrentAmmo (Variables|Default|GetWeaponComponent)))
  (Variables|Default|SetCurentAmmo (Variables|Default|GetStoredAmmo))
  (Variables|Default|SetStoredAmmo (LocalVariables|GetTemp)))

(fn UpdateAmmoUI
  (bind _foundwidgets (Class|WidgetBlueprintLibrary|GetAllWidgetswithInterface "/Game/Blueprint/UI/BPI_UIAmmo.BPI_UIAmmo_C" false))
  (Class|BPIUIAmmo|GetCurrentAmmo(Message) (Utilities|Array|Get(acopy) _foundwidgets) (Variables|/Game/Blueprint/Weapons/Components/COM_BaseWeaponLogic.COM_BaseWeaponLogic_C|GetCurrentAmmo (Variables|Default|GetWeaponComponent)))
  (return))