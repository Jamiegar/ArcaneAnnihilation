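; Base projectile actor with configurable colour, speed and bouncing, which damages actors that have a COM_Health component, excluding its instigator.
; On overlap, a small sphere trace and closest-bone lookup detect head hits for double damage, headshot sound and effect, then the projectile destroys itself.
; Surface hits spawn a tinted Niagara cloud and short-lived splat decal.
; Projectiles also expire after a lifespan or once velocity reaches zero.
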(event OnComponentBeginOverlap(Sphere)
  (params (OverlappedComponent :type Primitive%20Component%20Object%20Reference) (OtherActor :type Actor%20Object%20Reference) (OtherComp :type Primitive%20Component%20Object%20Reference) (OtherBodyIndex :type Integer) (bFromSweep :type Boolean) (SweepResult :type Hit%20Result%20Structure%20%28by%20ref%29))
  (bind _returnvalue (Transformation|GetActorLocation))
  (bind _damageamount (Variables|Default|GetDamageAmount))
  (Utilities|IsValid (Actor|GetComponentbyClass OtherActor "/Game/Blueprint/COM_Health.COM_Health_C")
    (:Is%20Valid
      (if (not (== OtherActor (Variables|Default|GetDamageInstigator)))
        (bind (_outhit _returnvalue_2) (Collision|SphereTraceByChannel _returnvalue _returnvalue 5.0 "TraceTypeQuery4" false (Utilities|Array|MakeArray self) "None"))
        (if _returnvalue_2
          (if (and (or (== (.ReturnValue (Class|SkinnedMeshComponent|FindClosestBoneK2 (Actor|GetComponentbyClass (.HitActor (Collision|BreakHitResult _outhit)) "/Script/Engine.SkeletalMeshComponent") (.ImpactNormal (Collision|BreakHitResult _outhit)) 0.0)) "Head") (== (.ReturnValue (Class|SkinnedMeshComponent|FindClosestBoneK2 (Actor|GetComponentbyClass (.HitActor (Collision|BreakHitResult _outhit)) "/Script/Engine.SkeletalMeshComponent") (.ImpactNormal (Collision|BreakHitResult _outhit)) 0.0)) "HeadTop_End")) (Utilities|IsValid (Actor|GetComponentbyClass (.HitActor (Collision|BreakHitResult _outhit)) "/Script/Engine.SkeletalMeshComponent")))
            (Audio|PlaySoundatLocation "/Game/ExternalAssets_Ungraded/Ultimate_SFX/Gore_Sounds_Pro/Wavs/Head_exploding/SC_Headshot.SC_Headshot" (.Location (Collision|BreakHitResult _outhit)) "0, 0, 0" 1.0 1.0 0.0 0 0 0 0)
            (Niagara|SpawnSystematLocation "/Game/Art/VFX/Systems/NS_Headshot.NS_Headshot" (.Location (Collision|BreakHitResult _outhit))))
          (Class|BPIAnyDamage|AnyDamage(Message) OtherActor (Math|Float|SelectFloat (* _damageamount 2.0) _damageamount (and (or (== (.ReturnValue (Class|SkinnedMeshComponent|FindClosestBoneK2 (Actor|GetComponentbyClass (.HitActor (Collision|BreakHitResult _outhit)) "/Script/Engine.SkeletalMeshComponent") (.ImpactNormal (Collision|BreakHitResult _outhit)) 0.0)) "Head") (== (.ReturnValue (Class|SkinnedMeshComponent|FindClosestBoneK2 (Actor|GetComponentbyClass (.HitActor (Collision|BreakHitResult _outhit)) "/Script/Engine.SkeletalMeshComponent") (.ImpactNormal (Collision|BreakHitResult _outhit)) 0.0)) "HeadTop_End")) (Utilities|IsValid (Actor|GetComponentbyClass (.HitActor (Collision|BreakHitResult _outhit)) "/Script/Engine.SkeletalMeshComponent")))) (Variables|Default|GetDamageType) (Variables|Default|GetDamageInstigator))
          (Actor|DestroyActor)
          (else
            (Class|BPIAnyDamage|AnyDamage(Message) OtherActor (Variables|Default|GetDamageAmount) (Variables|Default|GetDamageType) (Variables|Default|GetDamageInstigator))
            (Actor|DestroyActor)))))))

(event OnComponentHit(Sphere)
  (params (HitComponent :type Primitive%20Component%20Object%20Reference) (OtherActor :type Actor%20Object%20Reference) (OtherComp :type Primitive%20Component%20Object%20Reference) (NormalImpulse :type Vector :default "0, 0, 0") (Hit :type Hit%20Result%20Structure%20%28by%20ref%29))
  (bind (_bblockinghit _binitialoverlap _time _distance _location _impactpoint _normal _impactnormal) (Collision|BreakHitResult Hit))
  ;[1 1 1] Test Tai, Probs not write xD - Dan B
  (bind _returnvalue (Niagara|SpawnSystematLocation "/Game/Art/VFX/Systems/NS_BulletCloud.NS_BulletCloud" _impactpoint (Math|Conversions|RotationFromXVector _impactnormal)))
  (Niagara|SetNiagaraVariable(LinearColor) _returnvalue "Colour" (Variables|Default|GetProjectileColour))
  (bind _returnvalue_2 (Rendering|Decal|SpawnDecalatLocation "/Game/Art/Decals/M_DecalSplat.M_DecalSplat" "22.000000,22.000000,22.000000" _impactpoint (Math|Conversions|RotationFromXVector _impactnormal) 1.5))
  (bind _returnvalue_3 (Rendering|Material|CreateDynamicMaterialInstance _returnvalue_2 :!class /Script/Engine.DecalComponent))
  (Rendering|Material|SetVectorParameterValue _returnvalue_3 "Colour" (Variables|Default|GetProjectileColour) :!class /Script/Engine.MaterialInstanceDynamic))

(event Custom|Enemy)

(event EventBeginPlay
  (Actor|SetLifeSpan 1e+01))

(event EventTick
  (params (DeltaSeconds :type Float%20%28single-precision%29))
  (if (Utilities|Operators|EqualEqual :A (Variables|/Script/Engine.MovementComponent|GetVelocity (Variables|Default|GetProjectileMovement)))
    (Actor|DestroyActor)))

(fn ConstructionScript
  (bind _projectilemovement (Variables|Default|GetProjectileMovement))
  (bind _output_get (Variables|/Script/Engine.ProjectileMovementComponent|SetMaxSpeed _projectilemovement (+ (Variables|Default|GetForwardSpeed) (Variables|Default|GetProjectileSpeed))))
  (Variables|/Script/Engine.ProjectileMovementComponent|SetInitialSpeed _projectilemovement _output_get)
  (Rendering|Material|SetCustomPrimitiveDataVector3 (Variables|Default|GetSphere1) 1 (Math|Conversions|ToVector(LinearColor) (Variables|Default|GetProjectileColour)))
  (Variables|/Script/Engine.ProjectileMovementComponent|SetbShouldBounce (Variables|Default|GetProjectileMovement) (Variables|Default|GetShouldBounce)))