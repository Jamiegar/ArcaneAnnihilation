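; Health pickup level element that heals an overlapping physics character through its COMHealth component and then hides for a cooldown.
; The Sphere overlap gives health, turns off collision and mesh visibility, and starts a one-shot timer, presumably for reactivation.
; SetActive, also run on BeginPlay, restores both and spawns a randomly rotated Niagara effect.
; Both SetActive and SetInactive set the Active flag to false.
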(event OnComponentBeginOverlap(Sphere)
  (params (OverlappedComponent :type Primitive%20Component%20Object%20Reference) (OtherActor :type Actor%20Object%20Reference) (OtherComp :type Primitive%20Component%20Object%20Reference) (OtherBodyIndex :type Integer) (bFromSweep :type Boolean) (SweepResult :type Hit%20Result%20Structure%20%28by%20ref%29))
  (bind _character (Class|BPICharacter|GetPhysicsCharacter(Message) OtherActor))
  (Utilities|IsValid _character
    (:Is%20Valid
      (Default|GainHealth (Variables|/Game/Blueprint/Character/BP_PhysicsCharcter.BP_PhysicsCharcter_C|GetCOM_Health _character) (Variables|Health|GetHealthToGive))
      (CallFunction|SetInactive)
      (Utilities|Time|SetTimerbyEvent (EventDispatchers|CreateEvent :!event Custom|SetActive) (Variables|Health|GetCooldown)))))

(event Custom|SetInactive
  (Variables|Default|SetActive false)
  (Collision|SetCollisionEnabled (Variables|Default|GetSphere) "NoCollision")
  (Rendering|SetVisibility (Variables|Default|GetStaticMesh) false true))

(event Custom|SetActive
  (Variables|Default|SetActive false)
  (Collision|SetCollisionEnabled (Variables|Default|GetSphere) "QueryOnly")
  (Rendering|SetVisibility (Variables|Default|GetStaticMesh) true false)
  (Niagara|SpawnSystematLocation "/Game/Art/VFX/Systems/NS_HealthSpawn.NS_HealthSpawn" (Transformation|GetActorLocation) (Math|Random|RandomRotator true)))

(event EventBeginPlay
  (CallFunction|SetActive))

(fn ConstructionScript)