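; Level portal actor that sends a character to the level named by LevelName.
; When a BPI_Character actor overlaps the capsule, it plays a portal sound and fades screen and audio to white, then opens that level.
; This only runs while LevelStreaming is off; no streaming path is implemented, and a node to disable movement input is left unconnected.
; The construction script applies PortalMaterial to the PortalTXT component.
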(event OnComponentBeginOverlap(Capsule)
  (params (OverlappedComponent :type Primitive%20Component%20Object%20Reference) (OtherActor :type Actor%20Object%20Reference) (OtherComp :type Primitive%20Component%20Object%20Reference) (OtherBodyIndex :type Integer) (bFromSweep :type Boolean) (SweepResult :type Hit%20Result%20Structure%20%28by%20ref%29))
  (if (not (Variables|Debug|GetLevelStreaming))
    (if (Utilities|DoesObjectImplementInterface OtherActor "/Game/Blueprint/Interfaces/BPI_Character.BPI_Character_C")
      (Audio|PlaySoundatLocation "/Game/Blueprint/Sound/Waves_Cues/S_Portal_Cue.S_Portal_Cue" (Transformation|GetWorldLocation (Variables|Default|GetPortalTXT)) "0, 0, 0" 1.0 1.0 3.0 0 0 0 0)
      (CallFunction|StartScreenFade 0.0 1.0 2.0 "(R=1.000000,G=1.000000,B=1.000000,A=1.000000)" true true (delegate Custom|OnScreenFadeComplete)))))

(event Custom|OnScreenFadeComplete
  (Game|OpenLevel(byName) (Variables|PortalVar|GetLevel%20Name)))

(fn ConstructionScript
  (Rendering|Material|SetMaterial (Variables|Default|GetPortalTXT) 0 (Variables|PortalVar|GetPortalMaterial)))