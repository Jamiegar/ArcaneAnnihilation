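; BP_HoverObject is a level element actor that displays a selectable static mesh and bobs it vertically.
; On BeginPlay it applies the ObjChoice mesh and plays the Floating timeline.
; Each timeline update adds a Z offset to the mesh's current world location, so movement is cumulative.
; The offset blends between negative and positive random bounds by the track value, re-rolled every update for uneven motion.
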(event EventBeginPlay
  (bind _staticmesh (Variables|Default|GetStaticMesh))
  (bind _returnvalue (Transformation|GetWorldLocation _staticmesh))
  (Components|StaticMesh|SetStaticMesh (Variables|Default|GetStaticMesh) (Variables|Default|GetObjChoice))
  (bind _newtrack_0 (Timeline|Floating Play)
    (:Update
      (Transformation|SetActorLocation (Math|Vector|MakeVector (.x _returnvalue) (.y _returnvalue) (+ (.z _returnvalue) (Math|Float|Lerp (Math|Random|RandomFloatinRange -2.0 -1.0) (Math|Random|RandomFloatinRange 2.0 1.0) _newtrack_0))) false false))))

(fn ConstructionScript)