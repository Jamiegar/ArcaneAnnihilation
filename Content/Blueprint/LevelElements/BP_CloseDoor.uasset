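; BP_CloseDoor is a level element door that moves vertically once when something first overlaps its trigger box.
; The overlap passes through a DoOnce to OBJMove, which plays the MoveOBJ timeline, setting the mesh's world Z to the curve's absolute value while keeping X and Y.
; The box component is destroyed when the timeline finishes, and the construction script applies the configurable Mesh to the static mesh.
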(event OnComponentBeginOverlap(Box)
  (params (OverlappedComponent :type Primitive%20Component%20Object%20Reference) (OtherActor :type Actor%20Object%20Reference) (OtherComp :type Primitive%20Component%20Object%20Reference) (OtherBodyIndex :type Integer) (bFromSweep :type Boolean) (SweepResult :type Hit%20Result%20Structure%20%28by%20ref%29))
  (Utilities|FlowControl|DoOnce false
    (:Completed
      (CallFunction|OBJMove))))

(event Custom|OBJ%20Move
  (bind _staticmesh (Variables|Default|GetStaticMesh))
  (bind _returnvalue (Transformation|GetWorldLocation _staticmesh))
  (bind _z_movement (Timeline|Move%20OBJ PlayFromStart)
    (:Update
      (Transformation|SetWorldLocation _staticmesh (Math|Vector|MakeVector (.x _returnvalue) (.y _returnvalue) _z_movement) false false))
    (:Finished
      (Components|DestroyComponent (Variables|Default|GetBox)))))

(fn ConstructionScript
  (Components|StaticMesh|SetStaticMesh (Variables|Default|GetStaticMesh) (Variables|Default|GetMesh)))