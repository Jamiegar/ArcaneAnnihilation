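; BP_Target is a damageable level element that is destroyed when its health component reports death from incoming damage.
; BeginPlay initializes the COMHealth component's message, and AnyDamage passes the damage amount to that component's LoseHealth.
; A true result calls Dead to destroy the actor, while otherwise Fire-type damage triggers FireDamage on itself.
; The construction script's assignment of Health to MaxHealth is unconnected and never runs.
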(event Custom|Dead
  (Actor|DestroyActor))

(event EventAnyDamage
  (params (DamageAmount :type Float%20%28double-precision%29) (DamageType :type ENUM_DamageType%20Enum :default "NewEnumerator2") (Instigator :type Actor%20Object%20Reference))
  (bind _dead (Default|LoseHealth (Variables|Default|GetCOM_Health) DamageAmount))
  (if _dead
    (CallFunction|Dead)
    (else
      (switch Utilities|FlowControl|Switch|SwitchonENUM_DamageType DamageType
        (:NewEnumerator0
          (CallFunction|FireDamage self))))))

(event EventBeginPlay
  (Class|BPIInitalizable|Init(Message) (Variables|Default|GetCOM_Health)))

(fn ConstructionScript)