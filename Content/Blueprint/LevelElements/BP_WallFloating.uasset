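; BP_WallFloating is a level element whose Cube component bobs vertically around its placed position.
; On BeginPlay it stores endpoints slightly above and below the Cube's relative location, then starts the Bob timeline.
; Each timeline update lerps between the upper and lower endpoints and teleports the Cube there without sweeping.
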(event EventBeginPlay
  (Variables|Default|SetStartingPos (+ (Variables|/Script/Engine.SceneComponent|GetRelativeLocation (Variables|Default|GetCube)) "0.000000,0.000000,25.000000"))
  (Variables|Default|SetTargetPos (- (Variables|/Script/Engine.SceneComponent|GetRelativeLocation (Variables|Default|GetCube)) "0.000000,0.000000,25.000000"))
  (bind _alpha (Timeline|Bob PlayFromStart)
    (:Update
      (Transformation|SetRelativeLocation (Variables|Default|GetCube) (Math|Vector|Lerp(Vector) (Variables|Default|GetStartingPos) (Variables|Default|GetTargetPos) _alpha) false true))))

(fn ConstructionScript)