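; BP_Swarmer is a swarm enemy that runs the Swarm_BT behavior tree on its AI controller at BeginPlay.
; Attack Player does a debug-drawn box trace just ahead and damages any BP_PhysicsCharcter it hits, then calls Stop Attack.
; Stop Attack fires AttackStop and switches the blackboard States enum; a missed trace never reaches it.
; Death extends the parent's logic by removing the swarmer from the WaveManager's CombatDirector.
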(event EventBeginPlay
  (AI|RunBehaviorTree (AI|GetAIController self) "/Game/Blueprint/AI/BehaviourTree/Swarm_BT.Swarm_BT"))

(fn ConstructionScript
  (|CallParentFunction))

(fn AttackPlayer
  (bind _returnvalue (Transformation|GetActorLocation))
  (bind _returnvalue_2 (Transformation|GetActorRotation))
  (bind _returnvalue_3 (- _returnvalue "0.000000,0.000000,10.000000"))
  (bind _outhit (Collision|BoxTraceByChannel _returnvalue_3 (+ _returnvalue_3 (Math|Vector|RotateVector "50.000000,0.000000,0.000000" _returnvalue_2)) "300.000000,10.000000,50.000000" _returnvalue_2 "TraceTypeQuery1" false 0 "ForDuration"))
  (bind _asbp_physics_charcter (Utilities|Casting|CastToBP_PhysicsCharcter (.HitActor (Collision|BreakHitResult _outhit))))
  (Class|BPIAnyDamage|AnyDamage(Message) _asbp_physics_charcter 1e+01 "NewEnumerator2")
  (Development|PrintString "Hit")
  (CallFunction|StopAttack))

(fn StopAttack
  (bind _self self)
  (bind _returnvalue (AI|GetAIController _self))
  (bind _returnvalue_2 (AI|GetBlackboard _returnvalue))
  (Default|CallAttackStop)
  (Utilities|IsValid _returnvalue_2
    (:Is%20Valid
      (AI|Components|Blackboard|SetValueasEnum _returnvalue_2 (Utilities|Name|MakeLiteralName "States") (Utilities|Enum|LiteralenumE_SwarmerStates "NewEnumerator2")))
    (:Is%20Not%20Valid
      (Development|PrintString "found ya"))))

(fn Death
  (|CallParentFunction)
  (Default|RemoveSwarmer (Variables|/Game/Blueprint/GameMode/Managers/BP_WaveManager.BP_WaveManager_C|GetCombat%20Director (Variables|Default|GetWave%20Manager)) self))