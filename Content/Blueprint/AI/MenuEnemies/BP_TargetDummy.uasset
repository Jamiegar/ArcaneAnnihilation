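; BP_TargetDummy is a target dummy enemy, filed under menu enemies, that has its spawner respawn it when it leaves play.
; Init stores the Spawn reference and initializes COMHealth, whose MaxHealth the construction script sets from Health.
; EndPlay calls Respawn on that stored spawner.
; Death is overridden as empty, with the parent call left disconnected, so the inherited death logic does not run.
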(event Custom|Init
  (params (Spawn :type BP%20Menu%20Enemy%20Spawn%20Object%20Reference))
  (Variables|Default|SetSpawn Spawn)
  (Class|BPIInitalizable|Init(Message) (Variables|Default|GetCOM_Health)))

(event Collision|EventActorBeginOverlap
  (params (OtherActor :type Actor%20Object%20Reference)))

(event EventTick
  (params (DeltaSeconds :type Float%20%28single-precision%29)))

(event EventEndPlay
  (params (EndPlayReason :type EEndPlayReason%20Enum :default "Destroyed"))
  (Default|Respawn (Variables|Default|GetSpawn)))

(fn ConstructionScript
  (|CallParentFunction)
  (Variables|/Game/Blueprint/COM_Health.COM_Health_C|SetMaxHealth (Variables|Default|GetCOM_Health) (Variables|Default|GetHealth)))

(fn Death)