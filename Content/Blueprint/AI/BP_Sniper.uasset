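; BP_Sniper is an AI sniper enemy that runs the Sniper_BT behavior tree on BeginPlay.
; AttackPlayer calls RangeCheck, which line-traces along control rotation and randomly offsets the aim point by EnemyAccuracy.
; It then box-traces to that point and sends random damage to any BP_PhysicsCharcter hit, with debug drawing and print.
; StopAttack clears the attacking flag and resets the blackboard's attack and state keys.
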(event EventBeginPlay
  (AI|RunBehaviorTree (AI|GetAIController self) "/Game/Blueprint/AI/BehaviourTree/Sniper_BT.Sniper_BT"))

(fn ConstructionScript
  (|CallParentFunction))

(fn AttackPlayer
  (Variables|Default|SetAttacking? true)
  (CallFunction|RangeCheck)
  (bind _outhit (Collision|BoxTraceByChannel (Transformation|GetActorLocation) (Variables|Default|GetEnd) "300.000000,10.000000,50.000000" (Transformation|GetActorRotation) "TraceTypeQuery1" false 0 "ForDuration"))
  (bind _asbp_physics_charcter (Utilities|Casting|CastToBP_PhysicsCharcter (.HitActor (Collision|BreakHitResult _outhit))))
  (Class|BPIAnyDamage|AnyDamage(Message) _asbp_physics_charcter (Math|Random|RandomFloatinRange 0.0 3e+01) "NewEnumerator2")
  (Development|PrintString "Sniper Hit"))

(fn StopAttack
  (Variables|Default|SetAttacking? false)
  (AI|Components|Blackboard|SetValueasBool (AI|GetBlackboard (AI|GetAIController self)) (Utilities|Name|MakeLiteralName "isattacking?") false)
  (AI|Components|Blackboard|SetValueasEnum (AI|GetBlackboard (AI|GetAIController self)) (Utilities|Name|MakeLiteralName "States") (Utilities|Enum|LiteralenumE_SniperStates "NewEnumerator0")))

(fn RangeCheck
  (bind _returnvalue (Transformation|GetActorLocation))
  (bind _enemy_accuracy (Variables|Default|GetEnemy%20Accuracy))
  (bind _returnvalue_2 (* _enemy_accuracy -5.0))
  (bind _returnvalue_3 (Math|Random|RandomFloatinRange _returnvalue_2 _enemy_accuracy))
  (bind (_outhit _returnvalue_4) (Collision|LineTraceForObjects _returnvalue (+ _returnvalue (* (Math|Vector|GetForwardVector (Pawn|GetControlRotation :!class /Script/Engine.Pawn)) (Variables|Default|GetRange))) (Utilities|Array|MakeArray "ObjectTypeQuery1" "ObjectTypeQuery2" "ObjectTypeQuery3") false 0 "ForDuration" true "(R=1.000000,G=0.000000,B=0.000000,A=1.000000)" "(R=0.000000,G=1.000000,B=0.000000,A=1.000000)" 0.5))
  (Variables|Default|SetEnd (Math|Vector|MakeVector (+ (.X (Math|Vector|BreakVector (select _returnvalue_4 (+ (.ImpactPoint (Collision|BreakHitResult _outhit)) (Math|Vector|GetForwardVector (Pawn|GetControlRotation :!class /Script/Engine.Pawn))) (.TraceEnd (Collision|BreakHitResult _outhit))))) _returnvalue_3) (+ (.Y (Math|Vector|BreakVector (select _returnvalue_4 (+ (.ImpactPoint (Collision|BreakHitResult _outhit)) (Math|Vector|GetForwardVector (Pawn|GetControlRotation :!class /Script/Engine.Pawn))) (.TraceEnd (Collision|BreakHitResult _outhit))))) _returnvalue_3) (+ (.Z (Math|Vector|BreakVector (select _returnvalue_4 (+ (.ImpactPoint (Collision|BreakHitResult _outhit)) (Math|Vector|GetForwardVector (Pawn|GetControlRotation :!class /Script/Engine.Pawn))) (.TraceEnd (Collision|BreakHitResult _outhit))))) _returnvalue_3))))