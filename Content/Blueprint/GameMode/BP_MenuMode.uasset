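; Game mode for the menu that hides the mouse cursor on BeginPlay and starts a sequence of game-state changes.
; The Initalize event sets up the player manager and advances the state, and PreGame advances it again, then unpauses after a short delay.
; StartGame and EndGame are empty, and the WBP_GameStart widget creation is disconnected, so it never runs.
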(event EventBeginPlay
  (Variables|/Script/Engine.PlayerController|SetbShowMouseCursor (Game|GetPlayerController 0) false)
  (CallFunction|ChangeGameState "NewEnumerator0"))

(event EventInitalize
  (CallFunction|SetupManager "/Game/Blueprint/GameMode/Managers/BP_PlayerManager.BP_PlayerManager_C" (Variables|Default|GetPlayerManager))
  (CallFunction|ChangeGameState "NewEnumerator1"))

(event EventPreGame
  (CallFunction|ChangeGameState "NewEnumerator2")
  (Utilities|FlowControl|Delay 0.2)
  (Game|SetGamePaused false))

(event EventStartGame)

(event EventEndGame)

(fn ConstructionScript)