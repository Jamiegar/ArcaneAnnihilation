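; Game mode for Arcane Annihilation that drives match flow through Initalize, Pre-Game, Start Game and End Game states.
; ChangeGameState broadcasts each change and runs its handler; initialization finds and initializes the level's player and wave managers.
; Pre-game optionally waits on a countdown; each later state notifies BPI_CurrentGoal widgets.
; Advancing to Start Game and starting wave rounds happen inside those widget loops, so both fire per widget.
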(event Custom|Initalize
  (CallFunction|SetupManager "/Game/Blueprint/GameMode/Managers/BP_PlayerManager.BP_PlayerManager_C" (Variables|Default|GetPlayerManager))
  (CallFunction|SetupManager "/Game/Blueprint/GameMode/Managers/BP_WaveManager.BP_WaveManager_C" (Variables|Default|GetWaveManager))
  (CallFunction|ChangeGameState "NewEnumerator1"))

(event Custom|PreGame
  (if (Variables|Default|GetAllowCountdown)
    (CallFunction|StartCountdownWidget (delegate Custom|OnCountdownEnded))
    (else
      (bind _foundwidgets (Class|WidgetBlueprintLibrary|GetAllWidgetswithInterface "/Game/Blueprint/UI/BPI_CurrentGoal.BPI_CurrentGoal_C" false))
      (for _array_element _foundwidgets
        (Utilities|IsValid _array_element
          (:Is%20Valid
            (Class|BPICurrentGoal|GetCurretnGoal(Message) _array_element (Variables|Default|GetCurrentGameState)))
          (:Is%20Not%20Valid
            _))
        (CallFunction|ChangeGameState "NewEnumerator2")))))

(event Custom|StartGame
  (bind _foundwidgets (Class|WidgetBlueprintLibrary|GetAllWidgetswithInterface "/Game/Blueprint/UI/BPI_CurrentGoal.BPI_CurrentGoal_C" false))
  (for _array_element _foundwidgets
    (Utilities|IsValid _array_element
      (:Is%20Valid
        (Class|BPICurrentGoal|GetCurretnGoal(Message) _array_element (Variables|Default|GetCurrentGameState)))
      (:Is%20Not%20Valid
        _))
    (Default|StartRound (Variables|Default|GetWaveManager))))

(event Custom|EndGame
  (bind _foundwidgets (Class|WidgetBlueprintLibrary|GetAllWidgetswithInterface "/Game/Blueprint/UI/BPI_CurrentGoal.BPI_CurrentGoal_C" false))
  (for _array_element _foundwidgets
    (Utilities|IsValid _array_element
      (:Is%20Valid
        (Class|BPICurrentGoal|GetCurretnGoal(Message) _array_element (Variables|Default|GetCurrentGameState))))))

(event Custom|OnCountdownEnded
  (bind _foundwidgets (Class|WidgetBlueprintLibrary|GetAllWidgetswithInterface "/Game/Blueprint/UI/BPI_CurrentGoal.BPI_CurrentGoal_C" false))
  (for _array_element _foundwidgets
    (Utilities|IsValid _array_element
      (:Is%20Valid
        (Class|BPICurrentGoal|GetCurretnGoal(Message) _array_element (Variables|Default|GetCurrentGameState)))
      (:Is%20Not%20Valid
        _))
    (CallFunction|ChangeGameState "NewEnumerator2")))

(event EventBeginPlay
  (CallFunction|ChangeGameState "NewEnumerator0"))

(fn ConstructionScript)

(fn SetupManager
  (params (ManagerType :type BP%20Managers%20Class%20Reference) (ManagerVariable :type BP%20Managers%20Object%20Reference%20%28by%20ref%29))
  (bind _returnvalue (Actor|GetActorOfClass ManagerType))
  (bind _output_get (LocalVariables|SetTempManager _returnvalue))
  (Utilities|IsValid _output_get
    (:Is%20Valid
      (Class|BPIInitalizable|Init(Message) (LocalVariables|GetTempManager))
      (|SetBy-RefVar ManagerVariable (LocalVariables|GetTempManager)))
    (:Is%20Not%20Valid
      (Development|PrintString (Utilities|String|Append "Manager: " (Utilities|GetClassDisplayName ManagerType) " Not In level") true true "(R=1.000000,G=0.000000,B=0.015484,A=1.000000)"))))

(fn ChangeGameState
  (params (CurrentGameState :type E_GameState%20Enum :default "NewEnumerator0"))
  (bind _output_get (Variables|Default|SetCurrentGameState CurrentGameState))
  (Default|CallOnStateChnaged _output_get)
  (switch Utilities|FlowControl|Switch|SwitchonE_GameState _output_get
    (:NewEnumerator0
      (CallFunction|Initalize))
    (:NewEnumerator1
      (CallFunction|PreGame))
    (:NewEnumerator2
      (CallFunction|StartGame))
    (:NewEnumerator3
      (CallFunction|EndGame))))

(fn GetArcaneGameMode
  (return self))