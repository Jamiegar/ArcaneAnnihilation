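; BP_PlayerManager is a manager that sets up the local player: controller, pawn and possession.
; Init removes player 0, creates a new player, initializes its controller and sets game-only input.
; It then spawns and initializes a BP_PhysicsCharcter at the stored PlayerStart, and the controller possesses it.
; GetPlayerStarts caches a single PlayerStart actor, but Init does not call it.
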(event EventInit
  (CallFunction|CreatePlayerController)
  (CallFunction|CreatePawn)
  (CallFunction|PossessPawn))

(fn ConstructionScript
  (|CallParentFunction))

(fn CreatePlayerController
  (Class|GameplayStatics|RemovePlayer (Game|GetPlayerController 0) false)
  (bind _returnvalue (Class|GameplayStatics|CreatePlayer -1))
  (bind _controller (Class|BPIController|GetController(Message) _returnvalue))
  (bind _output_get (Variables|Default|SetController _controller))
  (Class|BPIInitalizable|Init(Message) _output_get)
  (Input|SetInputModeGameOnly _output_get false))

(fn CreatePawn
  (bind _returnvalue (Game|SpawnActorfromClass "/Game/Blueprint/Character/BP_PhysicsCharcter.BP_PhysicsCharcter_C" (Transformation|GetActorTransform (Variables|PreGame|GetPlayerStart)) "Undefined" 0 0))
  (bind _output_get (Variables|Default|SetPlayerPawn _returnvalue))
  (Class|BPIInitalizable|Init(Message) _output_get))

(fn GetPlayerStarts
  (bind _returnvalue (Actor|GetActorOfClass "/Script/Engine.PlayerStart"))
  (Variables|PreGame|SetPlayerStart _returnvalue))

(fn PossessPawn
  (Pawn|Possess (Variables|Default|GetController) (Variables|Default|GetPlayerPawn)))