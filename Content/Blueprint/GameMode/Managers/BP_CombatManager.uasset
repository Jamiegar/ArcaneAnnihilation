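; Combat manager that staggers enemy attacks by choosing which sniper or swarmer attacks next.
; Random grades are stored in maps, and the highest-graded enemy is picked, then given a new grade after attacking.
; A gated looping timer calls AttackPlayer on snipers, prioritising the most recently registered one.
; Swarmers are seeded with grades at init and attack through a blackboard flag on their AI controller.
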(event Custom|Init%20Combat%20Manager
  (for _array_element (Variables|Default|GetSwarmers)
    (Utilities|Map|Add (Variables|Default|GetSwarmer%20Grading) _array_element (Math|Random|RandomFloatinRange 1.0 5.0)))
  (Utilities|Time|SetTimerbyEvent (EventDispatchers|CreateEvent :!event Custom|Swarmer%20Attack%20Trigger) 1.0 true))

(event Custom|Swarmer%20Attack%20Trigger
  (bind _highest_enemy (CallFunction|PickSwarmer))
  (Utilities|IsValid _highest_enemy
    (:Is%20Valid
      (AI|Components|Blackboard|SetValueasBool (AI|GetBlackboard (AI|GetAIController _highest_enemy)) (Utilities|Name|MakeLiteralName "canAttack?") true)
      (Utilities|Map|Add (Variables|Default|GetSwarmer%20Grading) _highest_enemy (Math|Random|RandomFloatinRange 1.0 5.0)))))

(event Custom|Selector
  (bind _returnvalue (Utilities|Time|SetTimerbyEvent (delegate Custom|Select) 2.0 true))
  (Variables|Default|SetTimer _returnvalue)
  (Utilities|FlowControl|Gate true) ; enters at Open
)

(event Custom|Select
  (Utilities|FlowControl|Gate true
    (:Exit
      (Utilities|IsValid (Variables|Default|GetReady%20Sniper)
        (:Is%20Valid
          (if (Utilities|Array|ContainsItem (Variables|Default|GetSnipers) (Variables|Default|GetReady%20Sniper))
            (Default|AttackPlayer (Variables|Default|GetReady%20Sniper))
            (Utilities|Time|ClearandInvalidateTimerbyHandle (Variables|Default|GetTimer))
            (Utilities|Time|SetTimerbyEvent (delegate Custom|Selector) 2.0)
            (Variables|Default|SetReady%20Sniper 0)))
        (:Is%20Not%20Valid
          (bind _highest_sniper (CallFunction|PickSniper))
          (Utilities|IsValid _highest_sniper
            (:Is%20Valid
              (Default|AttackPlayer _highest_sniper)
              (Utilities|Map|Add (Variables|Default|GetSniper%20Grading) _highest_sniper (Math|Random|RandomFloatinRange 1.0 5.0)))))))))

(event Custom|New%20Enemy
  (params (New%20Sniper%20Enemy :type BP%20Sniper%20Object%20Reference%20%28by%20ref%29))
  (Utilities|Array|AddUnique (Variables|Default|GetSnipers) New%20Sniper%20Enemy)
  (Variables|Default|SetReady%20Sniper New%20Sniper%20Enemy)
  (CallFunction|ActivateManager))

(event Custom|Activate%20Manager
  (Utilities|FlowControl|DoOnce false
    (:Completed
      (CallFunction|Selector))))

(event Custom|Remove%20Enemy
  (params (Enemy%20to%20Remove :type BP%20Sniper%20Object%20Reference))
  (Utilities|Array|RemoveItem (Variables|Default|GetSnipers) Enemy%20to%20Remove)
  (if (Utilities|Array|IsEmpty (Variables|Default|GetSnipers))
    (Utilities|FlowControl|DoOnce false) ; enters at Reset
  ))

(event Custom|Stop%20Selector
  (Utilities|Time|ClearandInvalidateTimerbyHandle (Variables|Default|GetTimer))
  (Utilities|FlowControl|Gate true) ; enters at Close
)

(fn ConstructionScript)

(fn PickSwarmer
  (bind _keys (Utilities|Map|Keys (Variables|Default|GetSwarmer%20Grading)))
  (for _array_element _keys
    (if (>= (.Value (Utilities|Map|Find (Variables|Default|GetSwarmer%20Grading) _array_element)) (LocalVariables|GetLocal%20Highest))
      (LocalVariables|SetLocal%20Highest (.Value (Utilities|Map|Find (Variables|Default|GetSwarmer%20Grading) _array_element)))
      (LocalVariables|SetLocalHighest _array_element)))
  (return (LocalVariables|GetLocal%20Highest) (LocalVariables|GetLocalHighest)))

(fn PickSniper
  (bind _keys (Utilities|Map|Keys (Variables|Default|GetSniper%20Grading)))
  (for _array_element _keys
    (if (>= (.Value (Utilities|Map|Find (Variables|Default|GetSniper%20Grading) _array_element)) (LocalVariables|GetLocal%20Highest))
      (LocalVariables|SetLocal%20Highest (.Value (Utilities|Map|Find (Variables|Default|GetSniper%20Grading) _array_element)))
      (LocalVariables|SetLocal%20Highest%20Enemy _array_element)))
  (return (LocalVariables|GetLocal%20Highest) (LocalVariables|GetLocal%20Highest%20Enemy)))