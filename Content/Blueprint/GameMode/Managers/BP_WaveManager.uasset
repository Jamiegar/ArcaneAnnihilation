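; Wave manager that runs combat rounds, spawning enemy waves and tracking kills until each round completes.
; StartRound uses a curve over round number to mix difficulty tiers of wave data assets, loaded by folder through the Asset Registry.
; Random waves spawn at BP_EnemySpawn points; deaths update UI, outline the last stragglers via custom depth, then advance waves.
; Round completion activates a chest; the older PDA_Round selection still loads but its consumer is disconnected.
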(event Custom|Start%20Wave
  (bind _enemy_spawns (Variables|Default|GetEnemy%20Spawns))
  (bind _enemy_spawns_2 (Variables|Default|GetEnemy%20Spawns))
  (bind _returnvalue (Utilities|Array|LastIndex _enemy_spawns))
  (bind _returnvalue_2 (Math|Random|RandomIntegerinRange 0 _returnvalue))
  (bind _output (Utilities|Array|Get(acopy) _enemy_spawns_2 _returnvalue_2))
  (bind _returnvalue_3 (Transformation|GetActorTransform _output))
  (bind (_location _rotation) (Math|Transform|BreakTransform _returnvalue_3))
  ;[1 1 1] Waves
  (bind _output_get (Variables|Default|SetWaveToUse (.OutItem (Utilities|Array|Random (Variables|Default|GetWaves)))))
  (Utilities|IsValid _output_get
    (:Is%20Valid
      (for _array_element (Variables|/Game/Blueprint/AI/PDA_EnemyWave.PDA_EnemyWave_C|GetEnemies%20to%20Spawn _output_get)
        (bind _returnvalue_4 (Game|SpawnActorfromClass _array_element (Math|Transform|MakeTransform (Math|Vector|MakeVector (.x _location) (.y _location) (+ (.z _location) 5e+01)) _rotation "1.000000,1.000000,1.000000") "AlwaysSpawn" 0 0))
        (Default|InitAI _returnvalue_4 self)
        (Math|Integer|IncrementInt (Variables|Default|GetEnemies%20in%20Wave)))
      (CallFunction|UpdateEnemyUI)
      (Variables|Default|SetTotal%20Enemies (Variables|Default|GetEnemies%20in%20Wave))
      (Audio|PlaySound2D "/Game/SFX/MS_WaveStarted.MS_WaveStarted" 1.0 1.0 0.0 0 0))))

(event Custom|Check%20Wave%20Status
  ;[1 1 1] Waves
  (if (<= (Variables|Default|GetEnemies%20in%20Wave) 0)
    (CallFunction|WaveComplete)
    (elif (== (Variables|Default|GetEnemies%20in%20Wave) (Math|Integer|Clamp(Integer) (Math|Float|Round (* (Math|Conversions|ToFloat(Integer) (Variables|Default|GetTotal%20Enemies)) 0.25)) 3 500))
      (bind _outactors (Actor|GetAllActorsOfClass "/Game/Blueprint/AI/BP_BaseAI.BP_BaseAI_C"))
      (for _array_element _outactors
        (Utilities|IsValid _array_element
          (:Is%20Valid
            (if (not (Variables|/Game/Blueprint/AI/BP_BaseAI.BP_BaseAI_C|GetDead? _array_element))
              (Rendering|SetRenderCustomDepth (Variables|/Script/Engine.Character|GetMesh _array_element) true))))))))

(event Custom|Wave%20Complete
  ;[1 1 1] Waves
  (if (== (+ (Variables|Default|GetCurrent%20Wave) 1) (Variables|Default|GetTotal%20Waves))
    (Variables|Default|SetCurrent%20Wave 0)
    (CallFunction|RoundComplete)
    (else
      (Math|Integer|IncrementInt (Variables|Default|GetCurrent%20Wave)
        (:%20%20
          (Utilities|Array|Clear (Variables|/Game/Blueprint/GameMode/Managers/BP_CombatManager.BP_CombatManager_C|GetSwarmers (Variables|Default|GetCombat%20Director)))
          (Utilities|FlowControl|Delay 1.0)
          (CallFunction|StartWave))))))

(event Custom|Update%20Round%20UI
  ;[1 1 1] Update UI events
  (bind _foundwidgets (Class|WidgetBlueprintLibrary|GetAllWidgetswithInterface "/Game/Blueprint/GameMode/Managers/BPI_UIEnemyCounter.BPI_UIEnemyCounter_C" false))
  (Class|BPIUIEnemyCounter|GetRoundNumber(Message) _foundwidgets (Variables|Default|GetCurrent%20Round))
  (bind _returnvalue (UserInterface|CreateWidget "/Game/Blueprint/UI/Popup/WBP_RoundNumberPopup.WBP_RoundNumberPopup_C" 0 "Round Start" 1.2))
  (UserInterface|Viewport|AddtoViewport _returnvalue 0))

(event Custom|Start%20Round
  (bind _waves (Variables|Default|GetWaves))
  (Utilities|Array|Clear (Variables|Default|GetWaves))
  (Variables|Default|SetCurveValue (Math|Curves|GetFloatValue (Variables|Default|GetCurve) (Math|Conversions|ToFloat(Integer) (Variables|Default|GetCurrent%20Round))))
  (Utilities|FlowControl|Sequence
    (:then_0
      (if (< (Variables|Default|GetCurveValue) 5.0)
        (CallFunction|WaveLoop (Math|Float|Truncate (Variables|Default|GetCurveValue)) "EasyWaves")
        (elif (< (Variables|Default|GetCurveValue) 15.0)
          (CallFunction|WaveLoop (Math|Float|Truncate (* (Variables|Default|GetCurveValue) 0.4)) "EasyWaves")
          (CallFunction|WaveLoop (Math|Float|Truncate (* (Variables|Default|GetCurveValue) 0.6)) "MediumWaves")
          (elif (< (Variables|Default|GetCurveValue) 25.0)
            (CallFunction|WaveLoop (Math|Float|Truncate (* (Variables|Default|GetCurveValue) 0.4)) "MediumWaves")
            (CallFunction|WaveLoop (Math|Float|Truncate (* (Variables|Default|GetCurveValue) 0.6)) "HardWaves")))))
    (:then_1
      (Utilities|Array|Shuffle _waves)
      (Variables|Default|SetTotal%20Waves (Utilities|Array|Length _waves))
      (Variables|Default|SetCurrent%20Wave 0)
      (CallFunction|StartWave)
      (CallFunction|UpdateRoundUI))))

(event Custom|Update%20Enemy%20UI
  ;[1 1 1] Update UI events
  (bind _foundwidgets (Class|WidgetBlueprintLibrary|GetAllWidgetswithInterface "/Game/Blueprint/GameMode/Managers/BPI_UIEnemyCounter.BPI_UIEnemyCounter_C" false))
  (Class|BPIUIEnemyCounter|GetEnemyNumber(Message) _foundwidgets (Variables|Default|GetEnemies%20in%20Wave)))

(event Custom|Round%20Complete
  (Math|Integer|IncrementInt (Variables|Default|GetCurrent%20Round)
    (:%20%20
      (bind _returnvalue (UserInterface|CreateWidget "/Game/Blueprint/UI/Popup/WBP_RoundNumberPopup.WBP_RoundNumberPopup_C" 0 "Round Complete!" 1.2))
      (UserInterface|Viewport|AddtoViewport _returnvalue 0)
      (bind _outactors (Actor|GetAllActorsOfClass "/Game/Blueprint/Weapons/Pickup_World/BP_Chest.BP_Chest_C"))
      (Utilities|IsValid (Utilities|Array|Get(acopy) _outactors)
        (:Is%20Valid
          (Default|Activate (Utilities|Array|Get(acopy) _outactors) self)
          (Audio|PlaySound2D "/Game/SFX/MS_WaveEnded.MS_WaveEnded" 1.0 1.0 0.0 0 0))))))

(event Custom|Remove%20Enemy
  (params (Enemy%20that%20Died :type BP%20Base%20AI%20Object%20Reference))
  ;[1 1 1] Dead Enemy
  (Variables|/Game/Blueprint/AI/BP_BaseAI.BP_BaseAI_C|SetDead? Enemy%20that%20Died true)
  (Math|Integer|DecrementInt (Variables|Default|GetEnemies%20in%20Wave)
    (:%20%20
      (CallFunction|CheckWaveStatus)
      (CallFunction|UpdateEnemyUI))))

(event EventInit
  ;[1 1 1] Init
  (CallFunction|SelectRoundDifficulty (Variables|Default|GetCurrent%20Difficulty))
  (Variables|Default|SetCurrent%20Round 0)
  (bind _returnvalue (Game|SpawnActorfromClass "/Game/Blueprint/GameMode/Managers/BP_CombatManager.BP_CombatManager_C" (Math|Transform|MakeTransform "0, 0, 0" "0, 0, 0" "1.000000,1.000000,1.000000") "Undefined" 0 0))
  (Variables|Default|SetCombat%20Director _returnvalue)
  (bind _outactors (Actor|GetAllActorsOfClass "/Game/Blueprint/AI/BP_EnemySpawn.BP_EnemySpawn_C"))
  (for _array_element _outactors
    (Utilities|IsValid _array_element
      (:Is%20Valid
        (Utilities|Array|Add (Variables|Default|GetEnemy%20Spawns) _array_element)))))

(event EventTick
  (params (DeltaSeconds :type Float%20%28single-precision%29)))

(fn ConstructionScript)

(fn SelectRoundDifficulty
  (params (Round%20Level :type String))
  (bind _outassetdata (Class|AssetRegistry|GetAssetsbyPath (Class|AssetRegistryHelpers|GetAssetRegistry) (Utilities|String|StringToName (Utilities|String|Append "/Game/Blueprint/AI/Rounds/" Round%20Level)) false false))
  (bind _output_get (LocalVariables|SetNewLocalVar _outassetdata))
  (Utilities|Array|Shuffle _output_get)
  (for _array_element (LocalVariables|GetNewLocalVar)
    (bind _aspda_round (Utilities|Casting|CastToPDA_Round (Class|AssetRegistryHelpers|GetAsset _array_element)))
    (Utilities|IsValid _aspda_round
      (:Is%20Valid
        (Utilities|Array|Add (Variables|Default|GetRounds) _aspda_round)))))

(fn UpRoundDifficulty
  (params (Current%20Difficulty :type String))
  (switch string Current%20Difficulty
    (:EasyRounds
      (bind _output_get (Variables|Default|SetCurrent%20Difficulty "MediumRounds"))
      (return _output_get))
    (:MediumRounds
      (bind _output_get_2 (Variables|Default|SetCurrent%20Difficulty "HardRounds"))
      (return _output_get_2))
    (:HardRounds
      (bind _output_get_3 (Variables|Default|SetCurrent%20Difficulty "HardRounds"))
      (return _output_get_3))))

(fn SelectWaves
  (params (Round%20Level :type String))
  (bind _outassetdata (Class|AssetRegistry|GetAssetsbyPath (Class|AssetRegistryHelpers|GetAssetRegistry) (Utilities|String|StringToName (Utilities|String|Append "/Game/Blueprint/AI/Waves/" Round%20Level)) false false))
  (bind _output_get (LocalVariables|SetAssetData _outassetdata))
  (Utilities|Array|Shuffle _output_get)
  (bind _aspda_enemy_wave (Utilities|Casting|CastToPDA_EnemyWave (Class|AssetRegistryHelpers|GetAsset (Utilities|Array|Get(acopy) (LocalVariables|GetAssetData)))))
  (Utilities|IsValid _aspda_enemy_wave
    (:Is%20Valid
      (return _aspda_enemy_wave))))

(fn WaveLoop
  (params (LastIndex :type Integer) (Round%20Level :type String))
  (for _index (range 0 LastIndex)
    (bind _aspda_enemy_wave (CallFunction|SelectWaves Round%20Level))
    (Utilities|Array|Add (Variables|Default|GetWaves) _aspda_enemy_wave))
  (return))