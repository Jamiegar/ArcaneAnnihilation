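; Health component that tracks current and maximum health and a death flag for its owner.
; Init fills health to the maximum, GainHealth clamps to it, and getters expose the state.
; Lethal damage in LoseHealth fires OnDeath, sets IsDead and returns true, leaving the stored health unchanged.
; GainHealth broadcasts OnHealthAdded before applying the gain, so its NewHealth argument carries the old value.
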(event EventInit
  (Variables|Default|SetCurrentHealth (Variables|Default|GetMaxHealth)))

(fn GetCurrentHealth
  (return (Variables|Default|GetCurrentHealth)))

(fn GetMaxHealth
  (return (Variables|Default|GetMaxHealth)))

(fn LoseHealth
  (params (HealthToLose :type Float%20%28double-precision%29))
  (if (<= (- (Variables|Default|GetCurrentHealth) HealthToLose) 0.0)
    (Default|CallOnDeath)
    (Variables|Default|SetIsDead true)
    (return true)
    (else
      (Variables|Default|SetCurrentHealth (- (Variables|Default|GetCurrentHealth) HealthToLose))
      (return false))))

(fn GainHealth
  (params (HealthToGive :type Float%20%28double-precision%29))
  (Default|CallOnHealthAdded HealthToGive (Variables|Default|GetCurrentHealth))
  (if (> (+ (Variables|Default|GetCurrentHealth) HealthToGive) (Variables|Default|GetMaxHealth))
    (Variables|Default|SetCurrentHealth (Variables|Default|GetMaxHealth))
    (else
      (Variables|Default|SetCurrentHealth (+ (Variables|Default|GetCurrentHealth) HealthToGive)))))

(fn IsCharacterDead
  (return (Variables|Default|GetIsDead)))